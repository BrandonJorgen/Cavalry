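; BP_PlayerController is the VR player controller that routes motion controller input to the possessed BP_CavalryPlayerCharacter, cached on BeginPlay.
; Thumbstick axes drive the character's Move, Strafe and Rotate functions.
; Grab actions call Grab and Release on the left and right controllers.
; Valve Index grab axes do the same past a small threshold, using a DoOnce per hand so Release fires only once.
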(event EventBeginPlay
  (bind _asbp_cavalry_player_character (Utilities|Casting|CastToBP_CavalryPlayerCharacter (Pawn|GetControlledPawn)))
  (Variables|Default|SetPossessedCharacter _asbp_cavalry_player_character))

(event Input|ActionEvents|InputActionGrabLeft
  (params (Key :type Key%20Structure :default "None"))
  (bind _possessedcharacter (Variables|Default|GetPossessedCharacter))
  (bind _left_controller (Variables|/Game/Blueprints/BP_CavalryPlayerCharacter.BP_CavalryPlayerCharacter_C|GetLeft%20Controller _possessedcharacter))
  ;[0 0 0] Motion Controller Inputs
  ;;[0.07812 0.07812 0.07812] Left Controller Grab Input
  (:Pressed
    (Default|Grab _left_controller))
  (:Released
    (Default|Release _left_controller)))

(event Input|ActionEvents|InputActionGrabRight
  (params (Key :type Key%20Structure :default "None"))
  (bind _possessedcharacter (Variables|Default|GetPossessedCharacter))
  (bind _right_controller (Variables|/Game/Blueprints/BP_CavalryPlayerCharacter.BP_CavalryPlayerCharacter_C|GetRight%20Controller _possessedcharacter))
  ;[0 0 0] Motion Controller Inputs
  ;;[0.08854 0.08854 0.08854] Right Controller Grab Input
  (:Pressed
    (Default|Grab _right_controller))
  (:Released
    (Default|Release _right_controller)))

(event Input|AxisEvents|InputAxisGrabLeftIndex
  (params (AxisValue :type Float%20%28single-precision%29))
  (bind _possessedcharacter (Variables|Default|GetPossessedCharacter))
  (bind _left_controller (Variables|/Game/Blueprints/BP_CavalryPlayerCharacter.BP_CavalryPlayerCharacter_C|GetLeft%20Controller _possessedcharacter))
  ;[0 0 0] Motion Controller Inputs
  ;;[0.08854 0.08854 0.08854] Left Controller Valve Index Grab
  (if (> AxisValue 0.1)
    (Default|Grab _left_controller)
    (goto _label Reset)
    (else
      (Utilities|FlowControl|DoOnce false :!label _label
        (:Completed
          (Default|Release _left_controller))))))

(event Input|AxisEvents|InputAxisGrabRightIndex
  (params (AxisValue :type Float%20%28single-precision%29))
  (bind _possessedcharacter (Variables|Default|GetPossessedCharacter))
  (bind _right_controller (Variables|/Game/Blueprints/BP_CavalryPlayerCharacter.BP_CavalryPlayerCharacter_C|GetRight%20Controller _possessedcharacter))
  ;[0 0 0] Motion Controller Inputs
  ;;[0.0625 0.0625 0.0625] Right Controller Valve Index Grab
  (if (> AxisValue 0.1)
    (Default|Grab _right_controller)
    (goto _label Reset)
    (else
      (Utilities|FlowControl|DoOnce false :!label _label
        (:Completed
          (Default|Release _right_controller))))))

(event Input|AxisEvents|InputAxisLeftHorizontalAxis
  (params (AxisValue :type Float%20%28single-precision%29))
  ;[0 0 0] Motion Controller Inputs
  ;;[0.07292 0.07292 0.07292] Strafe Left and Right
  (Default|Strafe (Variables|Default|GetPossessedCharacter) AxisValue))

(event Input|AxisEvents|InputAxisLeftVerticalAxis
  (params (AxisValue :type Float%20%28single-precision%29))
  ;[0 0 0] Motion Controller Inputs
  ;;[0.08854 0.08854 0.08854] Move Forward and Backward
  (Default|Move (Variables|Default|GetPossessedCharacter) AxisValue))

(event Input|AxisEvents|InputAxisRightHorizontalAxis
  (params (AxisValue :type Float%20%28single-precision%29))
  ;[0 0 0] Motion Controller Inputs
  ;;[0.0625 0.0625 0.0625] Rotate Character
  (Default|Rotate (Variables|Default|GetPossessedCharacter) AxisValue))

(fn ConstructionScript)