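; Player gear rig for the Horseman characters, holding pistol, main weapon, tool and ammo grab trigger on mesh sockets.
; BeginPlay spawns and attaches an ammo trigger configured for the selected Horseman's weapon.
; CheckforTeleport disables physics and snaps ungrabbed weapons, plus the tool when also inactive, back to their sockets.
; Spawn chains for pistol, Horseman weapons and War's deployable shield are disconnected, so this graph never assigns those items.
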(event EventBeginPlay
  (bind _sm_fp_gear_whitebox (Variables|Default|GetSM_FP_Gear_Whitebox))
  (bind _returnvalue (Transformation|GetSocketLocation _sm_fp_gear_whitebox "Ammo_Trigger_Socket"))
  (Utilities|FlowControl|Sequence
    (:then_2
      ;[0 0 0] Spawn Ammo Grab Trigger
      (switch Utilities|FlowControl|Switch|SwitchonE_Horsemen (Variables|Default|GetHorsemanToSpawnFor)
        (:NewEnumerator0
          ;;[0.09412 0.09412 0.09412] Rifle Magazine Trigger
          (bind _returnvalue_2 (Game|SpawnActorfromClass "/Game/Blueprints/Characters/Gear/BP_GrabAmmoTrigger.BP_GrabAmmoTrigger_C" (Math|Transform|MakeTransform _returnvalue "0, 0, 0" "1,1,1") "Undefined" self "NewEnumerator2" 0))
          (bind _output_get (Variables|Default|SetAmmoTrigger _returnvalue_2))
          (Transformation|AttachActorToActor _output_get self "Ammo_Trigger_Socket" "SnapToTarget" "SnapToTarget" "SnapToTarget" false))
        (:NewEnumerator1
          ;;[0.09412 0.09412 0.09412] Shotgun Shell Trigger
          (bind _returnvalue_3 (Game|SpawnActorfromClass "/Game/Blueprints/Characters/Gear/BP_GrabAmmoTrigger.BP_GrabAmmoTrigger_C" (Math|Transform|MakeTransform _returnvalue "0, 0, 0" "1,1,1") "Undefined" self "NewEnumerator1" 0))
          (bind _output_get_2 (Variables|Default|SetAmmoTrigger _returnvalue_3))
          (Transformation|AttachActorToActor _output_get_2 self "Ammo_Trigger_Socket" "SnapToTarget" "SnapToTarget" "SnapToTarget" false))
        (:NewEnumerator2
          ;;[0.09412 0.09412 0.09412] DMR Magazine Trigger
          (bind _returnvalue_4 (Game|SpawnActorfromClass "/Game/Blueprints/Characters/Gear/BP_GrabAmmoTrigger.BP_GrabAmmoTrigger_C" (Math|Transform|MakeTransform _returnvalue "0, 0, 0" "1,1,1") "Undefined" self "NewEnumerator3" 0))
          (bind _output_get_3 (Variables|Default|SetAmmoTrigger _returnvalue_4))
          (Transformation|AttachActorToActor _output_get_3 self "Ammo_Trigger_Socket" "SnapToTarget" "SnapToTarget" "SnapToTarget" false))
        (:NewEnumerator3
          ;;[0.09412 0.09412 0.09412] SMG Magazine Trigger
          (bind _returnvalue_5 (Game|SpawnActorfromClass "/Game/Blueprints/Characters/Gear/BP_GrabAmmoTrigger.BP_GrabAmmoTrigger_C" (Math|Transform|MakeTransform _returnvalue "0, 0, 0" "1,1,1") "Undefined" self "NewEnumerator4" 0))
          (bind _output_get_4 (Variables|Default|SetAmmoTrigger _returnvalue_5))
          (Transformation|AttachActorToActor _output_get_4 self "Ammo_Trigger_Socket" "SnapToTarget" "SnapToTarget" "SnapToTarget" false))))))

(event EventCheckforTeleport
  (bind _tool (Variables|Default|GetTool))
  (bind _tool_2 (Variables|Default|GetTool))
  (bind _mainweapon (Variables|Default|GetMainWeapon))
  (bind _pistol (Variables|Default|GetPistol))
  ;[0 0 0] Teleporting items back to Gear
  (Utilities|FlowControl|Sequence
    (:then_0
      (if (not (Variables|/Game/Blueprints/Weapons/BP_Firearm_Base.BP_Firearm_Base_C|GetFirstHandGrabbed (Variables|Default|GetPistol)))
        (Physics|SetSimulatePhysics (Variables|/Game/Blueprints/Weapons/BP_Firearm_Base.BP_Firearm_Base_C|GetFirearm_SM _pistol) false)
        (Transformation|AttachActorToActor _pistol self "Pistol_Socket" "SnapToTarget" "SnapToTarget" "SnapToTarget" false)
        (Development|PrintString "[PLAYER GEAR] Pistol snapped back to socket")))
    (:then_1
      (if (not (Variables|/Game/Blueprints/Weapons/BP_Firearm_Base.BP_Firearm_Base_C|GetFirstHandGrabbed (Variables|Default|GetMainWeapon)))
        (Physics|SetSimulatePhysics (Variables|/Game/Blueprints/Weapons/BP_Firearm_Base.BP_Firearm_Base_C|GetFirearm_SM _mainweapon) false)
        (Transformation|AttachActorToActor _mainweapon self "Main_Weapon_Socket" "SnapToTarget" "SnapToTarget" "SnapToTarget" false)
        (Development|PrintString "[PLAYER GEAR] Main Weapon snapped back to socket")))
    (:then_2
      (if (not (Variables|/Game/Blueprints/Tools/BP_Tool_Base.BP_Tool_Base_C|GetisGrabbed _tool))
        (if (not (Variables|/Game/Blueprints/Tools/BP_Tool_Base.BP_Tool_Base_C|GettoolActivated _tool))
          (Physics|SetSimulatePhysics (Variables|/Game/Blueprints/Tools/BP_Tool_Base.BP_Tool_Base_C|GetTool_SkM _tool_2) false)
          (Transformation|AttachActorToActor _tool_2 self "Tool_Socket" "SnapToTarget" "SnapToTarget" "SnapToTarget" false)
          (Development|PrintString "[PLAYER GEAR] Tool snapped back to socket"))))))

(fn ConstructionScript)