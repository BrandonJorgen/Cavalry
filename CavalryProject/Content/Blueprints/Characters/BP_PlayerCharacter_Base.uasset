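; Base VR player character that spawns and attaches motion-controller hands, magnetic gear and HUD, with stick movement and snap or smooth turning.
; Tick keeps capsule and gear under the headset and triggers footstep audio by distance travelled.
; Authority-side damage drains shields, then counts health hits with temporary invulnerability until death disables hands, destroys gear and triggers the all-players-dead check.
; Also runs oracle voice tutorials and toggles night vision when Famine is present.
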(event Custom|ResetHitTimer
  ;[0 0 0] Taking Damage
  (Variables|Stats|SetrecentlyHit false))

(event Custom|Death
  (bind _left_controller (Variables|Default|GetLeft%20Controller))
  (bind _right_controller (Variables|Default|GetRight%20Controller))
  ;[0 0 0] Player Death
  (Collision|SetCollisionEnabled (Variables|/Game/VirtualRealityBP/Blueprints/BP_MotionController.BP_MotionController_C|GetGrabSphere _left_controller) "NoCollision")
  (Default|ReleaseActor _left_controller)
  (Default|HideHand _left_controller)
  (Collision|SetCollisionEnabled (Variables|/Game/VirtualRealityBP/Blueprints/BP_MotionController.BP_MotionController_C|GetGrabSphere _right_controller) "NoCollision")
  (Default|ReleaseActor _right_controller)
  (Default|HideHand _right_controller)
  (Variables|/Script/Engine.PostProcessComponent|SetbEnabled (Variables|Default|GetNight%20Vision%20PP) false)
  (Variables|/Script/Engine.PostProcessComponent|SetbEnabled (Variables|Default|GetPlayerDeath) true)
  (Actor|DestroyActor (Variables|Default|GetPlayerGear))
  (Utilities|Array|RemoveIndex (Variables|Actor|GetTags self))
  (Default|CallRemoveasTarget)
  (bind _asgs_cavalry (Utilities|Casting|CastToGS_Cavalry (Game|GetGameState)))
  (Default|AllPlayersDeadCheck _asgs_cavalry)
  ;[0 0 0] Showing the Death Widget
  (Default|DeathNote (Variables|Default|GetWidgetHandler))
  ;[1 0.03215 0.935] Death Oracle Audio
  (Audio|PlaySoundatLocation "/Game/SFX/Garbo_Sounds/Death_Oracle.Death_Oracle" (Transformation|GetWorldLocation (Variables|Default|GetCamera)) "0, 0, 0" 1.0 1.0 0.0 0 0 0))

(event Custom|Server_UpdateGearRotationPosition
  (bind _gearlocationbase (Variables|Default|GetGearLocationBase))
  ;[0 0 0] Gear Rotation and Position Update
  (Transformation|SetWorldRotation _gearlocationbase (Math|Rotator|MakeRotator 0.0 0.0 (.yaw (Transformation|GetWorldRotation (Variables|Default|GetCamera)))) false false)
  (Transformation|SetWorldLocation _gearlocationbase (Transformation|GetWorldLocation (Variables|Default|GetCamera)) false false))

(event Custom|Player_NightVision_Audio
  ;[1 0 1] Player Audio
  (Audio|PlaySoundatLocation "/Game/SFX/Placeholder_SFX/Nightvision_Placeholder/Night_Vision__PH_.Night_Vision__PH_" (Transformation|GetActorLocation) "0, 0, 0" 1.0 1.0 0.0 "/Game/SFX/NewSoundAttenuation.NewSoundAttenuation" 0 0))

(event Custom|Player_Hit_NoShield_Audio
  ;[1 0 1] Player Audio
  (Audio|PlaySoundatLocation "/Game/SFX/Placeholder_SFX/Grunt_Placeholders/Male_Player_Grunt.Male_Player_Grunt" (Transformation|GetActorLocation) "0, 0, 0" 1.0 1.0 0.0 0 0 0))

(event Custom|Player_Hit_Shield_Audio
  ;[1 0 1] Player Audio
)

(event Custom|Player_Walk_Audio
  (params (SurfaceType :type EPhysicalSurface%20Enum :default "SurfaceType_Default"))
  (bind _returnvalue (Transformation|GetActorLocation))
  ;[1 0 1] Player Audio
  (bind _returnvalue_2 (Class|FMODBlueprintStatics|PlayEventatLocation (Variables|Audio|GetPlayer_Walk_Event) (Transformation|GetActorTransform)))
  (Utilities|FlowControl|DoOnce false) ; enters at Reset
)

(event Custom|Player_Grab_Generic_Audio
  ;[1 0 1] Player Audio
)

(event Custom|Delay_Player_Walk_Audio
  (bind _returnvalue (Transformation|GetActorLocation))
  ;[1 0 1] Player Audio
  (Utilities|FlowControl|DoOnce false
    (:Completed
      (Utilities|FlowControl|Delay 0.4)
      (bind _outhit (Collision|LineTraceForObjects _returnvalue (- _returnvalue "0, 0,100.000000") (Utilities|Array|MakeArray "ObjectTypeQuery1" "ObjectTypeQuery2") false 0 "None"))
      (CallFunction|PlayerWalkAudio (Variables|/Script/PhysicsCore.PhysicalMaterial|GetSurfaceType (.physmat _outhit))))))

(event Custom|Run%20Tutorial
  (Utilities|FlowControl|DoOnce false :!label _label
    (:Completed
      (if (Variables|Tutorial|GetMag_Grab_Tuto)
        (if (Variables|Tutorial|GetGun_Load_Tuto)
          (if (Variables|Tutorial|GetCharge_Pull_Tuto)
            (if (Variables|Tutorial|GetEject_Mag_Tuto)
              _
              (else
                (Audio|PlaySoundatLocation "/Game/SFX/Garbo_Sounds/Eject_Magazine_Oracle.Eject_Magazine_Oracle" "0, 0, 0" "0, 0, 0" 1.0 1.0 0.0 0 0 0)
                (Variables|Tutorial|SetEject_Mag_Tuto true)
                (Utilities|FlowControl|Delay 8.0)))
            (if (Variables|Tutorial|GetFire_Mode_Tuto)
              _
              (else
                (Audio|PlaySoundatLocation "/Game/SFX/Garbo_Sounds/Fire_Mode_Oracle.Fire_Mode_Oracle" "0, 0, 0" "0, 0, 0" 1.0 1.0 0.0 0 0 0)
                (Variables|Tutorial|SetFire_Mode_Tuto true)
                (Utilities|FlowControl|Delay 6.0)))
            (if (not (Variables|Tutorial|GetIndicators_Tuto))
              (Audio|PlaySoundatLocation "/Game/SFX/Garbo_Sounds/Indicators_Oracle.Indicators_Oracle" "0, 0, 0" "0, 0, 0" 1.0 1.0 0.0 0 0 0)
              (Variables|Tutorial|SetIndicators_Tuto true))
            (else
              (Audio|PlaySoundatLocation "/Game/SFX/Garbo_Sounds/Charge_Handle_Pull_Oracle.Charge_Handle_Pull_Oracle" "0, 0, 0" "0, 0, 0" 1.0 1.0 0.0 0 0 0)
              (Variables|Tutorial|SetCharge_Pull_Tuto true)
              (Utilities|FlowControl|Delay 6.0)
              (goto _label Reset)))
          (else
            (Audio|PlaySoundatLocation "/Game/SFX/Garbo_Sounds/Gun_Load_Oracle.Gun_Load_Oracle" "0, 0, 0" "0, 0, 0" 1.0 1.0 0.0 0 0 0)
            (Variables|Tutorial|SetGun_Load_Tuto true)
            (Utilities|FlowControl|Delay 4.0)
            (goto _label Reset)))
        (else
          (Audio|PlaySoundatLocation "/Game/SFX/Garbo_Sounds/Magazine_Grab_Oracle.Magazine_Grab_Oracle" "0, 0, 0" "0, 0, 0" 1.0 1.0 0.0 0 0 0)
          (Variables|Tutorial|SetMag_Grab_Tuto true)
          (Utilities|FlowControl|Delay 9.0)
          (goto _label Reset))))))

(event Custom|Initialize%20Capsule%20Height
  ;[0 0 0] Grabbing Capsule Half-Height
)

(event Custom|Night%20Vision%20Trigger
  (bind _night_vision_pp (Variables|Default|GetNight%20Vision%20PP))
  ;[0 0 0] Famine Ability: Night vision
  (bind _returnvalue (Actor|GetActorOfClass "/Game/Blueprints/Characters/BPC_Famine.BPC_Famine_C"))
  (if (Utilities|IsValid _returnvalue)
    (Development|PrintString "Night Vision Trigger Success: Famine in Scene" true true "(R=0.000000,G=1.000000,B=0.193288,A=1.000000)")
    (Utilities|FlowControl|FlipFlop
      (:A
        (Variables|/Script/Engine.PostProcessComponent|SetbEnabled _night_vision_pp true)
        (Development|PrintString "Night Vision Trigger ON" true true "(R=0.000000,G=1.000000,B=0.193288,A=1.000000)"))
      (:B
        (Variables|/Script/Engine.PostProcessComponent|SetbEnabled _night_vision_pp false)
        (Development|PrintString "Night Vision Trigger OFF" true true "(R=1.000000,G=0.000000,B=0.000000,A=1.000000)")))
    (CallFunction|PlayerNightVisionAudio)
    (else
      (Development|PrintString "Night Vision Trigger Failure: Famine not in Scene" true true "(R=1.000000,G=0.000000,B=0.000000,A=1.000000)"))))

(event Custom|Server_UpdatePlayerCollisionPosition
  (bind _camera (Variables|Default|GetCamera))
  (bind _capsulecomponent (Variables|Collision|GetCapsuleComponent))
  (bind _returnvalue (Transformation|GetWorldLocation _camera))
  (bind _returnvalue_2 (Transformation|GetWorldLocation _capsulecomponent))
  (bind _returnvalue_3 (- _returnvalue _returnvalue_2))
  ;[0 0 0] Player collision position updating
  (Transformation|AddActorWorldOffset (Math|Vector|MakeVector (.x _returnvalue_3) (.y _returnvalue_3) 0.0) true)
  (Transformation|AddWorldOffset (Variables|Default|GetVR%20Origin) (Math|Vector|NegateVector (Math|Vector|MakeVector (.x _returnvalue_3) (.y _returnvalue_3) 0.0)) false false))

(event Custom|ResetShieldPercentage
  ;[0 0 0] Shield Percentage Reset
  (bind _asbp_magnetic_placement (Utilities|Casting|CastToBP_MagneticPlacement (Variables|/Script/Engine.ChildActorComponent|GetChildActor (Variables|/Game/Blueprints/Characters/Gear/BP_PlayerGear.BP_PlayerGear_C|GetMagnet%206 (Variables|Default|GetPlayerGear)))))
  (bind _asbpc_shield_recharger (Utilities|Casting|CastToBPC_ShieldRecharger (Variables|/Game/Blueprints/Tools/BP_MagneticPlacement.BP_MagneticPlacement_C|GetAttachedObject _asbp_magnetic_placement)))
  (Default|UpdateShields _asbpc_shield_recharger))

(event Custom|Server_SpawnHands
  (bind _returnvalue (Math|Transform|MakeTransform "0, 0, 0"))
  (bind _self self)
  ;[0 0 0] Motion Controller Spawn and Attach
  (Utilities|FlowControl|Sequence
    (:then_0
      (bind _returnvalue_2 (Game|SpawnActorfromClass "/Game/VirtualRealityBP/Blueprints/BP_MotionController.BP_MotionController_C" _returnvalue "AlwaysSpawn" _self "Left" 0))
      (Variables|Default|SetLeft%20Controller _returnvalue_2)
      (Transformation|AttachComponentToComponent _returnvalue_2 (Variables|Default|GetVR%20Origin) "None" "SnapToTarget" "SnapToTarget" "KeepWorld" false))
    (:then_1
      (bind _returnvalue_3 (Game|SpawnActorfromClass "/Game/VirtualRealityBP/Blueprints/BP_MotionController.BP_MotionController_C" _returnvalue "AlwaysSpawn" _self "Right" 0))
      (Variables|Default|SetRight%20Controller _returnvalue_3)
      (Transformation|AttachComponentToComponent _returnvalue_3 (Variables|Default|GetVR%20Origin) "None" "SnapToTarget" "SnapToTarget" "KeepWorld" false))))

(event Custom|Server_SpawnGear
  ;[0 0 0] Gear Spawning (default horseman is War)
  (bind _returnvalue (Game|SpawnActorfromClass "/Game/Blueprints/Characters/Gear/BP_PlayerGear.BP_PlayerGear_C" (Math|Transform|MakeTransform "0, 0, 0") "AlwaysSpawn" self (Variables|Default|GetHorseman%20to%20Spawn%20For) 0))
  (bind _output_get (Variables|Default|SetPlayerGear _returnvalue))
  (Transformation|AttachComponentToComponent _output_get (Variables|Default|GetGearLoction) "None" "SnapToTarget" "SnapToTarget" "SnapToTarget" false)
  (Variables|/Game/Blueprints/Characters/Gear/BP_PlayerGear.BP_PlayerGear_C|SetAttachedPlayer _returnvalue self))

(event Custom|SpawnHUD
  ;[0 0 0] HUD Spawning
  (bind _returnvalue (Game|SpawnActorfromClass "/Game/HUD/Widgets/Damage_Display/BP_HorsemenHUD.BP_HorsemenHUD_C" (Math|Transform|MakeTransform "0, 0, 0" "0, 0, 0" "0.100000,0.100000,0.100000") "AlwaysSpawn" self 0))
  (bind _output_get (Variables|Default|SetWidgetHandler _returnvalue))
  (Transformation|AttachComponentToComponent _output_get (Variables|Default|GetCamera) "None" "KeepRelative" "KeepRelative" "KeepRelative" false))

(event Custom|DisablePPVolumes
  ;[0 0 0] Disable Post Processing Volumes
  (Variables|/Script/Engine.PostProcessComponent|SetbEnabled (Variables|Default|GetNight%20Vision%20PP) false)
  (Variables|/Script/Engine.PostProcessComponent|SetbEnabled (Variables|Default|GetPlayerDeath) false))

(event EventBeginPlay
  (Utilities|FlowControl|Sequence
    (:then_0
      ;[0 0 0] Setup Player Height for Each HMD [Oculus, Odyssey, SteamVR]
      (switch name (Class|HeadMountedDisplayFunctionLibrary|GetHMDDeviceName)
        (:Oculus%20HMD
          _)
        (:Windows%20Mixed%20Reality
          _))
      (Class|HeadMountedDisplayFunctionLibrary|SetTrackingOrigin "Floor"))
    (:then_1
      (Utilities|FlowControl|Sequence
        (:then_0
          (CallFunction|ServerSpawnHands)
          (Variables|/Script/HeadMountedDisplay.MotionControllerComponent|SetPlayerIndex (Variables|/Game/VirtualRealityBP/Blueprints/BP_MotionController.BP_MotionController_C|GetMotionController (Variables|Default|GetLeft%20Controller)) 0)
          (Variables|/Script/HeadMountedDisplay.MotionControllerComponent|SetPlayerIndex (Variables|/Game/VirtualRealityBP/Blueprints/BP_MotionController.BP_MotionController_C|GetMotionController (Variables|Default|GetRight%20Controller)) 0))
        (:then_1
          (CallFunction|ServerSpawnGear))
        (:then_2
          (CallFunction|SpawnHUD))))
    (:then_2
      (CallFunction|DisablePPVolumes))
    (:then_3
      (Class|HeadMountedDisplayFunctionLibrary|SetTrackingOrigin "Floor"))
    (:then_4
      ;[0 0 0] Fade in
      (CameraFades|StartCameraFade :self (Game|GetPlayerCameraManager (Class|GameplayStatics|GetPlayerControllerID (Game|GetPlayerController 0))) :FromAlpha 1.0 :Duration 5.0))
    (:then_5
      (Utilities|FlowControl|Delay 1e+01)
      (if (not (Variables|Tutorial|GetMag_Grab_Tuto))
        (CallFunction|RunTutorial)))))

(event EventTakeDamage
  (params (DamageAmount :type Integer))
  ;[0 0 0] Taking Damage
  (Networking|SwitchHasAuthority
    (:Authority
      (if (not (Variables|Stats|GetrecentlyHit))
        (Variables|Stats|SetcurrentShields (- (Variables|Stats|GetcurrentShields) DamageAmount))
        (CallFunction|ResetShieldPercentage)
        (if (<= (Variables|Stats|GetcurrentShields) 0)
          (Variables|Stats|SetcurrentShields 0)
          (Math|Integer|IncrementInt (Variables|Stats|GethealthHits)
            (:%20%20
              (Variables|Stats|SetrecentlyHit true)
              (Utilities|Time|SetTimerbyEvent (delegate Custom|ResetHitTimer) 3.0)
              ;[0 0 0] Should player be dead?
              (if (>= (Variables|Stats|GethealthHits) (Variables|Stats|GetmaxHealthHits))
                (CallFunction|Death)
                (CallFunction|PlayerHitNoShieldAudio))))
          (else
            (CallFunction|PlayerHitShieldAudio)))))))

(event EventTick
  (params (DeltaSeconds :type Float%20%28single-precision%29))
  (bind _returnvalue (Transformation|GetActorLocation))
  ;[0 0 0] TICK
  (CallFunction|ServerUpdatePlayerCollisionPosition)
  (CallFunction|ServerUpdateGearRotationPosition)
  ;[0 0 0] Foot step audio tracking via distance instead of timing it out
  (Utilities|FlowControl|DoOnce false :!label _label
    (:Completed
      (if (Variables|Default|GetInitialPositionSaved)
        (Utilities|FlowControl|Delay 0.3)
        (if (> (Math|Vector|Distance(Vector) (Variables|Default|GetSavedPosition) _returnvalue) (Variables|Default|GetDistanceMin))
          (CallFunction|DelayPlayerWalkAudio)
          (Variables|Default|SetSavedPosition (Transformation|GetActorLocation))
          (goto _label Reset)
          (else
            (goto _label Reset)))
        (else
          (Variables|Default|SetSavedPosition _returnvalue)
          (Variables|Default|SetInitialPositionSaved true)
          (goto _label Reset))))))

(fn ConstructionScript)

(fn Movement
  (params (Value :type Float%20%28single-precision%29))
  (bind _returnvalue (Transformation|GetActorLocation))
  ;[0 0 0] Forward and Backward Movement
  (Pawn|Input|AddMovementInput (Math|Vector|GetForwardVector (Variables|Default|GetCamera)) Value false)
  (if (and (and (not (> Value 0.1)) (not (< Value -0.1))) (Math|Vector|NotEqual(Vector) (Variables|Default|GetSavedPosition) _returnvalue 1.0))
    (Variables|Default|SetSavedPosition _returnvalue)))

(fn Strafe
  (params (value :type Float%20%28single-precision%29))
  ;[1 1 1] Strafe Movement Input
  (Pawn|Input|AddMovementInput (Math|Vector|GetRightVector (Variables|Default|GetCamera)) value false))

(fn Rotation
  (params (value :type Float%20%28single-precision%29))
  ;[1 1 1] Rotation
  (if (Variables|Movement|GetbSmoothRotation)
    ;;[0.1562 0.1562 0.1562] Continuous Rotation
    (Transformation|SetActorRotation (Math|Rotator|MakeRotator 0.0 0.0 (+ (.yaw (Transformation|GetActorRotation)) (* value (Variables|Movement|GetSmooth%20Rotation%20Speed)))))
    (else
      (Class|Actor|AddActorWorldRotation (Math|Rotator|MakeRotator 0.0 0.0 (* (Math|Float|Sign(Float) value) (Variables|Movement|GetSnap%20Rotation%20Degrees)))))))