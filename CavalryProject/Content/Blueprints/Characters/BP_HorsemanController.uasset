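; Player controller for the VR Horseman character that caches its possessed BP_Horseman_Base and forwards motion controller input to it.
; Grab inputs grip and release per hand, the left stick moves and strafes, the right stick turns once per push past a deadzone, and left stick press triggers night vision.
; Each trigger clicks that hand's widget interaction and fires any gripped BP_Firearm_Base, with DoOnce limiting it to one shoot message per press.
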(event Custom|FindPossessedCharacter
  (bind _asbp_horseman_base (Utilities|Casting|CastToBP_Horseman_Base (Pawn|GetControlledPawn)))
  (Utilities|IsValid _asbp_horseman_base
    (:Is%20Valid
      (Variables|Default|SetpossessedCharacter _asbp_horseman_base))))

(event EventBeginPlay
  (CallFunction|FindPossessedCharacter))

(event Input|ActionEvents|InputActionGrabLeft
  (params (Key :type Key%20Structure :default "None"))
  (bind _possessedcharacter (Variables|Default|GetpossessedCharacter))
  (bind _leftmotioncontroller (Variables|/Script/VRExpansionPlugin.VRBaseCharacter|GetLeftMotionController _possessedcharacter))
  ;[0 0 0] Left Controller Gripping
  (:Pressed
    (Default|Grip _possessedcharacter _leftmotioncontroller (Variables|/Script/VRExpansionPlugin.VRBaseCharacter|GetRightMotionController _possessedcharacter) (Variables|/Game/Blueprints/Characters/BP_Horseman_Base.BP_Horseman_Base_C|GetLeft%20Grab%20Sphere _possessedcharacter)))
  (:Released
    (Default|Release _possessedcharacter _leftmotioncontroller)))

(event Input|ActionEvents|InputActionPrimaryTriggerLeft
  (params (Key :type Key%20Structure :default "None"))
  (bind _possessedcharacter (Variables|Default|GetpossessedCharacter))
  (bind _leftwidgetinteraction (Variables|/Game/Blueprints/Characters/BP_Horseman_Base.BP_Horseman_Base_C|GetLeftWidgetInteraction _possessedcharacter))
  ;[0 0 0] Left Primary Trigger
  (:Pressed
    (CallFunction|ManageLeftHWidInteract true _leftwidgetinteraction)
    (bind _grippedactorarray (Class|GripMotionControllerComponent|GetGrippedActors (Variables|/Script/VRExpansionPlugin.VRBaseCharacter|GetLeftMotionController _possessedcharacter)))
    (bind _asbp_firearm_base (Utilities|Casting|CastToBP_Firearm_Base (Utilities|Array|Get(acopy) _grippedactorarray)))
    (Utilities|FlowControl|DoOnce false :!label _label
      (:Completed
        (Class|BPIWeaponControls|Shoot(Message) _asbp_firearm_base "NewEnumerator1"))))
  (:Released
    (CallFunction|ManageLeftHWidInteract false _leftwidgetinteraction)
    (Class|BPIWeaponControls|ShootRelease(Message) _asbp_firearm_base)
    (goto _label Reset)))

(event Input|ActionEvents|InputActionPrimaryTriggerRight
  (params (Key :type Key%20Structure :default "None"))
  (bind _possessedcharacter (Variables|Default|GetpossessedCharacter))
  (bind _rightwidgetinteraction (Variables|/Game/Blueprints/Characters/BP_Horseman_Base.BP_Horseman_Base_C|GetRightWidgetInteraction _possessedcharacter))
  ;[0 0 0] Right Primary Trigger
  (:Pressed
    (CallFunction|ManageRightHWidInteract true _rightwidgetinteraction)
    (bind _grippedactorarray (Class|GripMotionControllerComponent|GetGrippedActors (Variables|/Script/VRExpansionPlugin.VRBaseCharacter|GetRightMotionController _possessedcharacter)))
    (bind _asbp_firearm_base (Utilities|Casting|CastToBP_Firearm_Base (Utilities|Array|Get(acopy) _grippedactorarray)))
    (Utilities|FlowControl|DoOnce false :!label _label
      (:Completed
        (Class|BPIWeaponControls|Shoot(Message) _asbp_firearm_base "NewEnumerator0"))))
  (:Released
    (CallFunction|ManageRightHWidInteract false _rightwidgetinteraction)
    (Class|BPIWeaponControls|ShootRelease(Message) _asbp_firearm_base)
    (goto _label Reset)))

(event Input|ActionEvents|InputActionGrabRight
  (params (Key :type Key%20Structure :default "None"))
  (bind _possessedcharacter (Variables|Default|GetpossessedCharacter))
  (bind _rightmotioncontroller (Variables|/Script/VRExpansionPlugin.VRBaseCharacter|GetRightMotionController _possessedcharacter))
  ;[0 0 0] Right Controller Gripping
  (:Pressed
    (Default|Grip _possessedcharacter _rightmotioncontroller (Variables|/Script/VRExpansionPlugin.VRBaseCharacter|GetLeftMotionController _possessedcharacter) (Variables|/Game/Blueprints/Characters/BP_Horseman_Base.BP_Horseman_Base_C|GetRight%20Grab%20Sphere _possessedcharacter)))
  (:Released
    (Default|Release _possessedcharacter _rightmotioncontroller)))

(event Input|ActionEvents|InputActionThumbstickPressLeft
  (params (Key :type Key%20Structure :default "None"))
  ;[0 0 0] Nightvision
  (:Pressed
    (Default|NightVisionTrigger (Variables|Default|GetpossessedCharacter))))

(event Input|AxisEvents|InputAxisMotionControllerThumbLeft_X
  (params (AxisValue :type Float%20%28single-precision%29))
  ;[0 0 0] Forward/Backward and Left/Right Movement
  (Default|Strafe (Variables|Default|GetpossessedCharacter) AxisValue))

(event Input|AxisEvents|InputAxisMotionControllerThumbLeft_Y
  (params (AxisValue :type Float%20%28single-precision%29))
  ;[0 0 0] Forward/Backward and Left/Right Movement
  (Default|Move (Variables|Default|GetpossessedCharacter) AxisValue))

(event Input|AxisEvents|InputAxisMotionControllerThumbRight_X
  (params (AxisValue :type Float%20%28single-precision%29))
  ;[0 0 0] Rotation
  (if (>= (Math|Float|Absolute(Float) AxisValue) (Variables|Default|GetTurn%20Deadzone))
    (Utilities|FlowControl|DoOnce false :!label _label
      (:Completed
        (Default|Rotation (Variables|Default|GetpossessedCharacter) AxisValue)))
    (else
      (goto _label Reset))))

(fn ConstructionScript)

(fn ManageLeftHWidInteract
  (params (Pressed? :type Boolean) (Wid_Interaction :type Widget%20Interaction%20Component%20Object%20Reference))
  (if Pressed?
    (if (== (Variables|/Script/UMG.WidgetInteractionComponent|GetPointerIndex Wid_Interaction) 0)
      (Variables|/Script/UMG.WidgetInteractionComponent|SetPointerIndex Wid_Interaction 1))
    (Class|WidgetInteractionComponent|PressPointerKey Wid_Interaction "LeftMouseButton")
    (else
      (Class|WidgetInteractionComponent|ReleasePointerKey Wid_Interaction "LeftMouseButton"))))

(fn ManageRightHWidInteract
  (params (Pressed? :type Boolean) (Wid_Interaction :type Widget%20Interaction%20Component%20Object%20Reference))
  (if Pressed?
    (Class|WidgetInteractionComponent|PressPointerKey Wid_Interaction "LeftMouseButton")
    (else
      (Class|WidgetInteractionComponent|ReleasePointerKey Wid_Interaction "LeftMouseButton"))))