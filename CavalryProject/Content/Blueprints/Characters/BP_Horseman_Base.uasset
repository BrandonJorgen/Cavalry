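; Base VR player pawn for the Horsemen, with per-HMD tracking setup, camera-relative movement, snap turning and a Famine-dependent night vision toggle.
; Motion controllers grip the nearest overlapping actor through VRGripInterface, snapping to slots and supporting two-handed grips where allowed.
; Authority-side damage drains shields, then counts health hits with a brief invulnerability window.
; Death drops held items, destroys gear, enables death post-processing, notifies GS_Cavalry and shows the death widget.
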(event Custom|ResetHitTimer
  ;[0 0 0] Taking Damage
  (Variables|Stats|SetrecentlyHit false))

(event Custom|HideHands
  ;[0 0 0] Hide Player hands
  (Rendering|SetOnlyOwnerSee (Variables|Default|GetLeft%20Hand%20SkM) true :!class /Script/Engine.PrimitiveComponent)
  (Rendering|SetOnlyOwnerSee (Variables|Default|GetRight%20Hand%20SkM) true :!class /Script/Engine.PrimitiveComponent))

(event Custom|Night%20Vision%20Trigger
  (bind _night_vision_pp (Variables|Default|GetNight%20Vision%20PP))
  ;[0 0 0] Famine Ability: Night vision
  (bind _returnvalue (Actor|GetActorOfClass "/Game/Blueprints/Characters/BPC_Famine.BPC_Famine_C"))
  (if (Utilities|IsValid _returnvalue)
    (Development|PrintString "Night Vision Trigger Success: Famine in Scene" true true "(R=0.000000,G=1.000000,B=0.193288,A=1.000000)")
    (Utilities|FlowControl|FlipFlop
      (:A
        (Variables|/Script/Engine.PostProcessComponent|SetbEnabled _night_vision_pp true)
        (Development|PrintString "Night Vision Trigger ON" true true "(R=0.000000,G=1.000000,B=0.193288,A=1.000000)"))
      (:B
        (Variables|/Script/Engine.PostProcessComponent|SetbEnabled _night_vision_pp false)
        (Development|PrintString "Night Vision Trigger OFF" true true "(R=1.000000,G=0.000000,B=0.000000,A=1.000000)")))
    (else
      (Development|PrintString "Night Vision Trigger Failure: Famine not in Scene" true true "(R=1.000000,G=0.000000,B=0.000000,A=1.000000)"))))

(event Custom|Death
  ;[0 0 0] Player Death
  (Collision|SetCollisionEnabled (Variables|Default|GetLeft%20Grab%20Sphere) "NoCollision")
  (Gripping|Release (Variables|Default|GetLeftMotionController))
  (CallFunction|HideHands)
  (Collision|SetCollisionEnabled (Variables|Default|GetRight%20Grab%20Sphere) "NoCollision")
  (Gripping|Release (Variables|Default|GetRightMotionController))
  (Variables|/Script/Engine.PostProcessComponent|SetbEnabled (Variables|Default|GetNight%20Vision%20PP) false)
  (Variables|/Script/Engine.PostProcessComponent|SetbEnabled (Variables|Default|GetPlayerDeath) true)
  (Actor|DestroyActor (Variables|Default|GetPlayerGear))
  (Utilities|Array|RemoveIndex (Variables|Default|GetTags self))
  (Default|CallRemoveasTarget)
  (bind _asgs_cavalry (Utilities|Casting|CastToGS_Cavalry (Game|GetGameState)))
  (Default|AllPlayersDeadCheck _asgs_cavalry)
  ;[0 0 0] Showing the Death Widget
  (Default|DeathNote (Variables|Default|GetWidgetHandler)))

(event Custom|ResetShieldPercentage
  ;[0 0 0] Shield Percentage Reset
  (bind _asbp_magnetic_placement (Utilities|Casting|CastToBP_MagneticPlacement (Variables|/Script/Engine.ChildActorComponent|GetChildActor (Variables|/Game/Blueprints/Characters/Gear/BP_PlayerGear.BP_PlayerGear_C|GetMagnet%208 (Variables|Default|GetPlayerGear)))))
  (bind _asbpc_shield_recharger (Utilities|Casting|CastToBPC_ShieldRecharger (Variables|/Game/Blueprints/Tools/BP_MagneticPlacement.BP_MagneticPlacement_C|GetAttachedObject _asbp_magnetic_placement)))
  (Default|UpdateShields _asbpc_shield_recharger))

(event Custom|DisablePPVolumes
  ;[0 0 0] Disable Post Processing Volumes
  (Variables|/Script/Engine.PostProcessComponent|SetbEnabled (Variables|Default|GetNight%20Vision%20PP) false)
  (Variables|/Script/Engine.PostProcessComponent|SetbEnabled (Variables|Default|GetPlayerDeath) false))

(event Custom|CustomEvent
  (params (DamageAmount :type Integer))
  ;[0 0 0] Taking Damage
  (Networking|SwitchHasAuthority
    (:Authority
      (if (not (Variables|Stats|GetrecentlyHit))
        (Variables|Stats|SetcurrentShields (- (Variables|Stats|GetcurrentShields) DamageAmount))
        (CallFunction|ResetShieldPercentage)
        (if (<= (Variables|Stats|GetcurrentShields) 0)
          (Variables|Stats|SetcurrentShields 0)
          (Math|Integer|IncrementInt (Variables|Stats|GethealthHits)
            (:%20%20
              (Variables|Stats|SetrecentlyHit true)
              (Utilities|Time|SetTimerbyEvent (delegate Custom|ResetHitTimer) 3.0)
              ;[0 0 0] Should player be dead?
              (if (>= (Variables|Stats|GethealthHits) (Variables|Stats|GetmaxHealthHits))
                (CallFunction|Death)))))))))

(event EventBeginPlay
  (Utilities|FlowControl|Sequence
    (:then_0
      ;[0 0 0] Setup Player Height for Each HMD [Oculus, Odyssey, SteamVR]
      (switch name (Class|HeadMountedDisplayFunctionLibrary|GetHMDDeviceName)
        (:Oculus%20HMD
          _)
        (:Windows%20Mixed%20Reality
          _))
      (Class|HeadMountedDisplayFunctionLibrary|SetTrackingOrigin "Floor"))
    (:then_1
      (CallFunction|DisablePPVolumes))
    (:then_2
      ;[0 0 0] Fade in
      (CameraFades|StartCameraFade :self (Game|GetPlayerCameraManager (Class|GameplayStatics|GetPlayerControllerID (Game|GetPlayerController 0))) :FromAlpha 1.0 :Duration 5.0))))

(fn ConstructionScript)

(fn Grip
  (params (GrippingHand :type Grip%20Motion%20Controller%20Component%20Object%20Reference) (OtherHand :type Grip%20Motion%20Controller%20Component%20Object%20Reference) (GrippingHandCollider :type Primitive%20Component%20Object%20Reference))
  (bind (_nearestobject _objectworldtransform) (Gripping|FindNearestObject GrippingHandCollider))
  (LocalVariables|SetNearestObject _nearestobject)
  (LocalVariables|SetObjectWorldTransform _objectworldtransform)
  (if (Class|GripMotionControllerComponent|GetIsObjectHeld OtherHand (LocalVariables|GetNearestObject))
    ;[0 0 0] Double Grip
    (bind _asvrgrip_interface (Utilities|Casting|CastToVRGripInterface (LocalVariables|GetNearestObject)))
    (bind _returnvalue (Class|VRGripInterface|AllowsMultipleGrips _asvrgrip_interface))
    (if _returnvalue
      (bind _returnvalue_2 (Class|VRGripInterface|DenyGripping(Message) (LocalVariables|GetNearestObject))) ; Check if the grip interface is telling us that\nthis object doesn't want to be gripped.
      (if (not _returnvalue_2)
        (bind (_bhadslotinrange _slotworldtransform _slotname) (Class|VRGripInterface|ClosestGripSlotinRange(Message) (LocalVariables|GetNearestObject) (Transformation|GetWorldLocation GrippingHand) true GrippingHand "None"))
        (if _bhadslotinrange
          (LocalVariables|SetSlotName _slotname)
          (Class|GripMotionControllerComponent|GripObjectbyInterface GrippingHand (LocalVariables|GetNearestObject) (select _bhadslotinrange (Math|Transform|MakeRelativeTransform (LocalVariables|GetObjectWorldTransform) _slotworldtransform) (Class|GripMotionControllerComponent|ConverttoControllerRelativeTransform GrippingHand (LocalVariables|GetObjectWorldTransform))) true "None" (LocalVariables|GetSlotName) _bhadslotinrange)
          (return))))
    (else
      ;[0 0 0] Single Grip
      (bind _returnvalue_3 (Class|VRGripInterface|DenyGripping(Message) (LocalVariables|GetNearestObject))) ; Check if the grip interface is telling us that\nthis object doesn't want to be gripped.
      (if _returnvalue_3
        (return)
        (else
          (bind (_bhadslotinrange_2 _slotworldtransform_2 _slotname_2) (Class|VRGripInterface|ClosestGripSlotinRange(Message) (LocalVariables|GetNearestObject) (Transformation|GetWorldLocation GrippingHand) false GrippingHand "None"))
          (if _bhadslotinrange_2
            (LocalVariables|SetSlotName _slotname_2)
            (Class|GripMotionControllerComponent|GripObjectbyInterface GrippingHand (LocalVariables|GetNearestObject) (select _bhadslotinrange_2 (Math|Transform|MakeRelativeTransform (LocalVariables|GetObjectWorldTransform) _slotworldtransform_2) (Class|GripMotionControllerComponent|ConverttoControllerRelativeTransform GrippingHand (LocalVariables|GetObjectWorldTransform))) true "None" (LocalVariables|GetSlotName) _bhadslotinrange_2)
            (return)))))))

(fn SecondGrip
  (params (NearestActor :type Actor%20Object%20Reference) (GrippingHand :type Grip%20Motion%20Controller%20Component%20Object%20Reference) (OtherHand :type Grip%20Motion%20Controller%20Component%20Object%20Reference) (RelativeSecondTransform :type Transform) (IsSlotGrip :type Boolean))
  (if (Utilities|DoesObjectImplementInterface NearestActor "/Script/VRExpansionPlugin.VRGripInterface")
    (bind _returnvalue (Class|VRGripInterface|SecondaryGripType(Message) NearestActor))
    (if (Gripping|CanSecondGrip NearestActor _returnvalue IsSlotGrip)
      (Class|GripMotionControllerComponent|AddSecondaryAttachmentPoint OtherHand NearestActor GrippingHand RelativeSecondTransform true 0.25 IsSlotGrip "None")
      (return)
      (else
        (return)))))

(fn CanSecondGrip
  (params (GripActor :type Actor%20Object%20Reference) (SecGripType :type ESecondaryGripType%20Enum :default "SG_None") (IsSlotGrip :type Boolean))
  (if (Utilities|Enum|Equal(Enum) SecGripType "SG_None")
    (return false)
    (elif (Utilities|DoesObjectImplementInterface GripActor "/Script/VRExpansionPlugin.VRGripInterface")
      (if IsSlotGrip
        (return true)
        (else
          ;[0 0 0] Redundancy so we make sure that second gripping works if we really need it to without a slot
          (switch Utilities|FlowControl|Switch|SwitchonESecondaryGripType SecGripType
            (:SG_None
              _)
            (:SG_Free
              (return true))
            (:SG_SlotOnly
              _)
            (:SG_Free_Retain
              (return true))
            (:SG_SlotOnly_Retain
              _)
            (:SG_FreeWithScaling_Retain
              (return true))
            (:SG_SlotOnlyWithScaling_Retain
              _)
            (:SG_Custom
              (return true))
            (:SG_ScalingOnly
              (return true)))
          (return false)))
      (else
        (return false)))))

(fn Release
  (params (ReleasingHand :type Grip%20Motion%20Controller%20Component%20Object%20Reference))
  (bind _griparray (Class|GripMotionControllerComponent|GetAllGrips ReleasingHand))
  (for _array_element _griparray
    (Class|GripMotionControllerComponent|DropObjectbyInterface ReleasingHand 0 (.GripID (Utilities|Struct|BreakBPActorGripInformation _array_element)) "0, 0, 0" "0, 0, 0")
    (return)))

(fn FindNearestObject
  (params (GripCollider :type Primitive%20Component%20Object%20Reference))
  (for _array_element (Collision|GetOverlappingActors GripCollider "/Script/Engine.Actor" :!class /Script/Engine.PrimitiveComponent)
    (if (< (Math|Vector|VectorLength (- (Transformation|GetActorLocation _array_element) (Transformation|GetWorldLocation GripCollider))) (Variables|Gripping|GetNearestOverlap))
      (Variables|Gripping|SetNearestOverlappingActor _array_element)
      (Variables|Gripping|SetNearestOverlap (Math|Vector|VectorLength (- (Transformation|GetActorLocation _array_element) (Transformation|GetWorldLocation GripCollider))))))
  (Utilities|IsValid (Variables|Gripping|GetNearestOverlappingActor)
    (:Is%20Valid
      (return (Variables|Gripping|GetNearestOverlappingActor) (Transformation|GetActorTransform (Variables|Gripping|GetNearestOverlappingActor))))))

(fn Move
  (params (Value :type Float%20%28single-precision%29))
  (Pawn|Input|AddMovementInput (Math|Vector|GetForwardVector (Variables|Default|GetVRReplicatedCamera)) Value false)
  (return))

(fn Strafe
  (params (Value :type Float%20%28single-precision%29))
  (Pawn|Input|AddMovementInput (Math|Vector|GetRightVector (Variables|Default|GetVRReplicatedCamera)) Value false)
  (return))

(fn Rotation
  (params (Value :type Float%20%28single-precision%29))
  (Class|VRBaseCharacterMovementComponent|PerformMoveActionSnapTurn (Variables|Default|GetVRMovementReference) (* (Math|Float|Sign(Float) Value) (Variables|Movement|GetSnap%20Rotation%20Degrees)) "VRMOVEACTION_Velocity_None" false false)
  (return))