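; BP_SCOREBOARD runs a timed shooting range round and displays score, countdown and high score.
; Taking damage starts the round, and a timeline drives the countdown text.
; AddtoScore calls are only counted while the round runs.
; When time expires, it shows the score as high score if it beats HighScoreINT, which is never updated here, then resets score and labels.
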(event Custom|updateScoreboard
  (Rendering|Components|TextRender|SetText (Variables|Default|GetScore) (Utilities|Text|ToText(Integer) (Variables|Default|GetScore_INT))))

(event Custom|AddScore
  (params (ScoreAddition :type Integer))
  (if (Variables|Default|GetRunning)
    (Variables|Default|SetScore_INT (+ ScoreAddition (Variables|Default|GetScore_INT)))
    (CallFunction|UpdateScoreboard)
    (Math|Integer|IncrementInt (Variables|Default|GetActiveHits))))

(event EventAddtoScore
  (params (Addition :type Integer))
  (CallFunction|AddScore Addition))

(event EventTakeDamageActor
  (params (DamageAmount :type Integer) (DamagingActor :type Actor%20Object%20Reference))
  (Variables|Default|SetRunning true)
  (Rendering|Components|TextRender|SetText (Variables|Default|GetStart) (Utilities|Text|MakeLiteralText "Shoot Targets"))
  (bind _timer_track (Timeline|countdown PlayFromStart)
    (:Update
      (Rendering|Components|TextRender|SetText (Variables|Default|GetStart) (Utilities|Text|ToText(Float) _timer_track "HalfToEven" false true 1 324 0 1)))
    (:Finished
      (Variables|Default|SetRunning false)
      (if (< (Variables|Default|GetHighScore_INT) (Variables|Default|GetScore_INT))
        (Rendering|Components|TextRender|SetText (Variables|Default|GetHighScore) (Utilities|Text|ToText(String) (Utilities|String|Append "/" (Utilities|String|ToString(Integer) (Variables|Default|GetScore_INT))))))
      (Variables|Default|SetScore_INT 0)
      (Rendering|Components|TextRender|SetText (Variables|Default|GetStart) (Utilities|Text|MakeLiteralText "Start"))
      (Rendering|Components|TextRender|SetText (Variables|Default|GetScore) (Utilities|Text|MakeLiteralText "00")))))

(fn ConstructionScript)