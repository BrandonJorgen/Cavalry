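; Shooting range target dummy that tips over when the TakeDamageActor event fires, then swings back up.
; Two chained timelines lerp the mesh's relative rotation toward its local down axis, then its local up axis, re-caching the start transform before each swing.
; A Moving flag ignores further hits until the second timeline finishes.
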(event EventTakeDamageActor
  (params (DamageAmount :type Integer) (DamagingPawn :type Pawn%20Object%20Reference))
  (if (not (Variables|Default|GetMoving))
    (Variables|Default|SetMoving true)
    (Variables|Default|SetBeginningPosition (Transformation|GetRelativeTransform (Variables|Default|GetTarget_Dummy_1)))
    (bind _newtrack_0 (Timeline|Timeline_0 PlayFromStart)
      (:Update
        (Transformation|SetRelativeTransform (Variables|Default|GetTarget_Dummy_1) (Math|Transform|Lerp(Transform) (Variables|Default|GetBeginningPosition) (Math|Transform|MakeTransform (.location (Variables|Default|GetBeginningPosition)) (Math|Conversions|RotationFromXVector (Math|Vector|RotateVector "0,0.000000,-90.000000" (.rotation (Variables|Default|GetBeginningPosition)))) (.scale (Variables|Default|GetBeginningPosition))) _newtrack_0) false false))
      (:Finished
        (Variables|Default|SetBeginningPosition (Transformation|GetRelativeTransform (Variables|Default|GetTarget_Dummy_1)))
        (bind _newtrack_0_2 (Timeline|Timeline_1 PlayFromStart)
          (:Update
            (Transformation|SetRelativeTransform (Variables|Default|GetTarget_Dummy_1) (Math|Transform|Lerp(Transform) (Variables|Default|GetBeginningPosition) (Math|Transform|MakeTransform (.location (Variables|Default|GetBeginningPosition)) (Math|Conversions|RotationFromXVector (Math|Vector|RotateVector "0,0.000000,90.000000" (.rotation (Variables|Default|GetBeginningPosition)))) (.scale (Variables|Default|GetBeginningPosition))) _newtrack_0_2) false false))
          (:Finished
            (Variables|Default|SetMoving false)))))))

(fn ConstructionScript)