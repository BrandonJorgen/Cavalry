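; VR grab component that snaps its owning object to a named socket on whatever component grabs it.
; Grab, when active, disables physics on the supplied mesh and attaches the root actor's root component to the socket.
; For a right-hand BP_MotionController it also adds a half-turn rotation to correct orientation.
; Release re-enables physics and detaches the actor, keeping its world transform.
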(event Custom|Grab
  (params (StaticMeshComponent :type Mesh%20Component%20Object%20Reference) (RootActor :type Actor%20Object%20Reference) (SocketName :type Name) (AttachTo :type Scene%20Component%20Object%20Reference))
  ;[0 0 0] Grabbing
  (if (Variables|Default|GetComponentActive)
    (bind _output_get (Variables|Default|SetStaticMeshComponent StaticMeshComponent))
    (bind _output_get_2 (Variables|Default|SetRootActor RootActor))
    (Physics|SetSimulatePhysics _output_get false)
    (Transformation|AttachComponentToComponent (VehicleSound|GetRootComponent _output_get_2) AttachTo SocketName "SnapToTarget" "SnapToTarget" "SnapToTarget" false)
    (bind _asbp_motion_controller (Utilities|Casting|CastToBP_MotionController (Components|GetOwner AttachTo)))
    (if (Utilities|Enum|Equal(Enum) (Variables|/Game/VirtualRealityBP/Blueprints/BP_MotionController.BP_MotionController_C|GetHand _asbp_motion_controller) "Right")
      (Transformation|SetWorldTransform (VehicleSound|GetRootComponent _output_get_2) (Math|Transform|MakeTransform (Transformation|GetWorldLocation (VehicleSound|GetRootComponent _output_get_2)) (Transformation|GetWorldRotation (VehicleSound|GetRootComponent _output_get_2)) "1,1,1") false false)
      (Transformation|AddRelativeRotation (VehicleSound|GetRootComponent _output_get_2) "0.000000,0.000000,180.000000" false false))))

(event Custom|Release
  ;[0 0 0] Releasing
  (Physics|SetSimulatePhysics (Variables|Default|GetStaticMeshComponent) true)
  (Transformation|DetachFromActor (Variables|Default|GetRootActor) "KeepWorld" "KeepWorld" "KeepWorld"))