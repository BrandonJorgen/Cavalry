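; Game State for Cavalry that tracks mission objectives, combat music and team wipes.
; BeginPlay caches hostages, enemies and the player controller count; all hostages rescued plus the server download stopped triggers the security lockdown after a delay.
; CheckForCombat starts or ends music on every player character based on whether any enemy is in combat.
; All players dying returns to MainMenu; the lockdown-lifted and missile-stopped events are empty stubs.
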(event Custom|Phase1CompletionCheck
  (if (and (Variables|Default|GetHostagesRescued) (Variables|Default|GetServerDonwloadStopped))
    (Utilities|FlowControl|Delay 2.0)
    (Default|CallSecurityLockdownStart)))

(event Custom|AllPlayersDeadCheck
  (bind _deadplayercount (Variables|Default|GetDeadPlayerCount))
  (Math|Integer|IncrementInt _deadplayercount
    (:%20%20
      (if (>= _deadplayercount (Variables|Default|GetPlayerCount))
        (Utilities|FlowControl|Delay 5.0)
        (Game|OpenLevel(byName) "MainMenu")))))

(event Custom|CheckForCombat
  ;[0 0 0] Music System
  (Variables|Default|SetPlayerInCombat false)
  (bind _array_element (Utilities|Array|ForEachLoopwithBreak (Variables|Default|GetEnemyArray) :!label _label)
    (:LoopBody
      (if (Variables|/Game/Blueprints/Enemies/BP_EnemyBase.BP_EnemyBase_C|GetInCombat _array_element)
        (Variables|Default|SetPlayerInCombat true)
        (goto _label Break)))
    (:Completed
      (if (Variables|Default|GetPlayerInCombat)
        (CallFunction|StartMusic)
        (else
          (CallFunction|MuteMusic))))))

(event Custom|MuteMusic
  ;[0 0 0] Music System
  (for _array_element (Variables|Default|GetPlayerArray)
    (bind _asbp_player_character_base (Utilities|Casting|CastToBP_PlayerCharacter_Base (Variables|/Script/Engine.PlayerState|GetPawnPrivate _array_element)))
    (Default|EndMusic _asbp_player_character_base)))

(event Custom|StartMusic
  ;[0 0 0] Music System
  (for _array_element (Variables|Default|GetPlayerArray)
    (bind _asbp_player_character_base (Utilities|Casting|CastToBP_PlayerCharacter_Base (Variables|/Script/Engine.PlayerState|GetPawnPrivate _array_element)))
    (Default|StartMusic _asbp_player_character_base)))

(event Custom|RemoveFromEnemyArray
  (params (Actor :type BP%20Enemy%20Base%20Object%20Reference))
  (Utilities|Array|RemoveItem (Variables|Default|GetEnemyArray) Actor))

(event EventBeginPlay
  (bind _outactors (Actor|GetAllActorsOfClass "/Game/Blueprints/LF-19/BP_HostageTest.BP_HostageTest_C"))
  (Variables|Default|SetHostageArray _outactors)
  (bind _outactors_2 (Actor|GetAllActorsOfClass "/Game/Blueprints/Characters/BP_CavalryController.BP_CavalryController_C"))
  (Variables|Default|SetPlayerCount (Utilities|Array|Length _outactors_2))
  (Variables|Default|SetDeadPlayerCount 0)
  (bind _outactors_3 (Actor|GetAllActorsOfClass "/Game/Blueprints/Enemies/BP_EnemyBase.BP_EnemyBase_C"))
  (Variables|Default|SetEnemyArray _outactors_3))

(event EventServerDownloadStopped
  (Variables|Default|SetServerDonwloadStopped true)
  (CallFunction|Phase1CompletionCheck))

(event EventHostageRescued
  (bind _result (Math|Integer|IncrementInt (Variables|Default|GetHostageRescueCount))
    (:%20%20
      (if (>= _result (Utilities|Array|Length (Variables|Default|GetHostageArray)))
        (Variables|Default|SetHostagesRescued true)
        (CallFunction|Phase1CompletionCheck)
        (Default|CallHostageObjectiveComplete)))))

(event EventSecurityLockdownLifted)

(event EventMissileLaunchStopped)

(fn ConstructionScript)