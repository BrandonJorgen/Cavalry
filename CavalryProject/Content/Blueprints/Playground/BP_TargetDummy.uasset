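; BP_TargetDummy is a playground target dummy that takes hits, dies and respawns its mesh.
; Each TakeDamage event removes one Health point, and at zero it destroys the DummySM component, clears TargetAlive and starts a one-shot timer.
; The timer calls SpawnTarget, which adds a new static mesh component and sets TargetAlive again, without restoring Health or reassigning DummySM.
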(event Custom|SpawnTarget
  ;[0 0 0] Spawn new target
  (AddComponent|AddStaticMeshComponent false)
  (Variables|Default|SettargetAlive true))

(event EventTakeDamage
  (params (DamageAmount :type Integer))
  ;[0 0 0] Take Damage
  (bind _output_get (Variables|Default|Sethealth (- (Variables|Default|Gethealth) 1)))
  ;[0 0 0] Check if enemy should be dead
  (if (== _output_get 0)
    (Components|DestroyComponent (Variables|Default|GetDummy_SM))
    (Variables|Default|SettargetAlive false)
    (Utilities|Time|SetTimerbyEvent (delegate Custom|SpawnTarget) 4.0)))

(fn ConstructionScript)