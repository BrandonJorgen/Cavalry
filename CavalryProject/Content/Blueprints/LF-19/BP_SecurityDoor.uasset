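; Security door actor that slides its mesh vertically between closed and open positions.
; BeginPlay caches the open height from the mesh's relative Z, then sets the starting state from IsClosed on authority only.
; A timeline lerps the mesh's relative Z, playing forward to open and reversing to close.
; Other Blueprints drive it through UpdateDoorState, which stores the new state and triggers the matching animation.
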(event Custom|DoorClose
  ;[1 1 1] Open/Close Animation
  (bind _up_lerp (Timeline|OpenTimeline Reverse)
    (:Update
      (Transformation|SetRelativeLocation (Variables|Default|GetDoor_SM) (Math|Vector|MakeVector 0.0 0.0 (Math|Float|Lerp 0.0 (Variables|Default|GetOpenHeight) _up_lerp)) false false))))

(event Custom|DoorOpen
  ;[1 1 1] Open/Close Animation
  (bind _up_lerp (Timeline|OpenTimeline Play)
    (:Update
      (Transformation|SetRelativeLocation (Variables|Default|GetDoor_SM) (Math|Vector|MakeVector 0.0 0.0 (Math|Float|Lerp 0.0 (Variables|Default|GetOpenHeight) _up_lerp)) false false))))

(event Custom|UpdateDoorState
  (params (State :type Boolean))
  ;[1 1 1] Used by other BPs to control the opening and closing of the door
  (bind _output_get (Variables|Default|SetIsClosed State))
  (if _output_get
    (CallFunction|DoorClose)
    (else
      (CallFunction|DoorOpen))))

(event EventBeginPlay
  ;[1 1 1] Setting of variables and determining what state the door is starting in
  (Variables|Default|SetOriginalLocation (Transformation|GetActorLocation))
  (Variables|Default|SetOpenHeight (+ (.z (.location (Transformation|GetRelativeTransform (Variables|Default|GetDoor_SM)))) 2.5e+02))
  (Networking|SwitchHasAuthority
    (:Authority
      (if (Variables|Default|GetIsClosed)
        (CallFunction|DoorClose)
        (else
          (CallFunction|DoorOpen))))))

(fn ConstructionScript)