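; BP_HostageTest is a test hostage actor that the player rescues by touching it.
; A Box component's overlap and hit events both check for the Player tag and share one rescue path.
; That path hides the skeletal mesh and placeholder text, turns off the mesh's collision, and calls HostageRescuedMessage on the GameState.
; The Box's own collision stays enabled, and nothing guards against repeat triggers.
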(event OnComponentHit(Box)
  (params (HitComponent :type Primitive%20Component%20Object%20Reference) (OtherActor :type Actor%20Object%20Reference) (OtherComp :type Primitive%20Component%20Object%20Reference) (NormalImpulse :type Vector :default "0, 0, 0") (Hit :type Hit%20Result%20Structure%20%28by%20ref%29))
  ;[0 0 0] Did a player touch the hostage
  (if (Actor|ActorHasTag OtherActor "Player")
    (CallFunction|DisableHostage)
    (Class|BPIGameStateCommunication|HostageRescued(Message) (Game|GetGameState))))

(event OnComponentBeginOverlap(Box)
  (params (OverlappedComponent :type Primitive%20Component%20Object%20Reference) (OtherActor :type Actor%20Object%20Reference) (OtherComp :type Primitive%20Component%20Object%20Reference) (OtherBodyIndex :type Integer) (bFromSweep :type Boolean) (SweepResult :type Hit%20Result%20Structure%20%28by%20ref%29))
  ;[0 0 0] Did a player touch the hostage
  (if (Actor|ActorHasTag OtherActor "Player")
    (CallFunction|DisableHostage)
    (Class|BPIGameStateCommunication|HostageRescued(Message) (Game|GetGameState))))

(event Custom|DisableHostage
  (bind _skeletalmesh (Variables|Default|GetSkeletalMesh))
  ;[0 0 0] Disable the hostage
  (Rendering|SetVisibility _skeletalmesh false false)
  (Collision|SetCollisionEnabled _skeletalmesh "NoCollision")
  (Rendering|SetVisibility (Variables|Default|GetPLACEHOLDERTEXT) false false)
  (Rendering|SetVisibility (Variables|Default|GetPLACEHOLDERTEXT2) false false)
  (Rendering|SetVisibility (Variables|Default|GetPLACEHOLDERTEXT1) false false))

(fn ConstructionScript)