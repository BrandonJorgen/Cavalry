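; Shootable laptop actor that, when shot, signals that a download has stopped and then explodes.
; The Shot event acts only with authority, calling the game state's download-stopped message before triggering ShotEvent.
; ShotEvent plays the explosion audio event at the laptop's transform and destroys the actor.
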(event Custom|ShotEvent
  (Class|FMODBlueprintStatics|PlayEventatLocation (Variables|Audio|GetLaptop_Explode_Event) (Transformation|GetActorTransform))
  (Actor|DestroyActor))

(event EventShot
  (Networking|SwitchHasAuthority
    (:Authority
      (Class|BPIGameStateCommunication|ServerDownloadStopped(Message) (Game|GetGameState))
      (CallFunction|ShotEvent))))

(fn ConstructionScript
  (|CallParentFunction))