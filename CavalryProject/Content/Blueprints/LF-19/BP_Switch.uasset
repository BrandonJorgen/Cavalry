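; BP_Switch is a switch actor with placeholder text feedback that shows whether it is locked.
; An overlap on Base_SM, handled only on authority, recolors the text red when IsLocked is set, otherwise green, then restores white after short delays.
; A DoOnce blocks retriggering until the sequence ends.
; The locked branch's intermediate white steps are immediately overwritten by red, and a comment marks the color logic for replacement with a material.
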(event OnComponentBeginOverlap(Base_SM)
  (params (OverlappedComponent :type Primitive%20Component%20Object%20Reference) (OtherActor :type Actor%20Object%20Reference) (OtherComp :type Primitive%20Component%20Object%20Reference) (OtherBodyIndex :type Integer) (bFromSweep :type Boolean) (SweepResult :type Hit%20Result%20Structure%20%28by%20ref%29))
  (Networking|SwitchHasAuthority
    (:Authority
      (CallFunction|PlaceholderTextChange))))

(event Custom|PlaceholderTextChange
  (Utilities|FlowControl|DoOnce false :!label _label
    (:Completed
      (if (Variables|Default|GetIsLocked)
        ;[0 0 0] This section should replaced with a material
        (Rendering|Components|TextRender|SetTextRenderColor (Variables|Default|GetPLACEHOLDER) (Math|Color|MakeColor 0 0 255 255))
        (Utilities|FlowControl|Delay 0.3)
        (Rendering|Components|TextRender|SetTextRenderColor (Variables|Default|GetPLACEHOLDER) (Math|Color|MakeColor 255 255 255 255))
        (Rendering|Components|TextRender|SetTextRenderColor (Variables|Default|GetPLACEHOLDER) (Math|Color|MakeColor 0 0 255 255))
        (Utilities|FlowControl|Delay 0.3)
        (Rendering|Components|TextRender|SetTextRenderColor (Variables|Default|GetPLACEHOLDER) (Math|Color|MakeColor 255 255 255 255))
        (Rendering|Components|TextRender|SetTextRenderColor (Variables|Default|GetPLACEHOLDER) (Math|Color|MakeColor 0 0 255 255))
        (Utilities|FlowControl|Delay 0.3)
        (Rendering|Components|TextRender|SetTextRenderColor (Variables|Default|GetPLACEHOLDER) (Math|Color|MakeColor 255 255 255 255))
        (goto _label Reset)
        (else
          (Rendering|Components|TextRender|SetTextRenderColor (Variables|Default|GetPLACEHOLDER) (Math|Color|MakeColor 0 255 0 255))
          (Utilities|FlowControl|Delay 1.0)
          (Rendering|Components|TextRender|SetTextRenderColor (Variables|Default|GetPLACEHOLDER) (Math|Color|MakeColor 255 255 255 255))
          (goto _label Reset))))))

(fn ConstructionScript)