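; VR pistol Blueprint, derived from a parent class, that handles one- and two-handed grabbing.
; The first grab attaches the gun and records owner and dominant hand.
; A second grab picks the slider or support socket by whichever collider is nearer the controller.
; Timelines act as update loops, moving the slide within limits from controller motion or applying recoil pitch during support grip, until the second hand releases.
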(event EventGrab
  (params (HandSocket :type Name :default "None") (AttachToMe :type Scene%20Component%20Object%20Reference) (Actor :type Actor%20Object%20Reference))
  (bind _recoilactual (Variables|Default|GetRecoilActual))
  (bind _slider_sm (Variables|Default|GetSlider_SM))
  (bind _sliderxmin (Variables|Default|GetSliderXMin))
  (bind _firearm_sm (Variables|Default|GetFirearm_SM))
  ;[0 0 0] Grabbing
  (if (Variables|Default|GetFirstHandGrabbed)
    ;;[0.1329 0.1329 0.1329] Which Collider is closer?
    (bind _asbp_motion_controller (Utilities|Casting|CastToBP_MotionController Actor))
    (if (< (Math|Vector|VectorLength (- (Transformation|GetWorldLocation (Variables|/Game/VirtualRealityBP/Blueprints/BP_MotionController.BP_MotionController_C|GetMotionController _asbp_motion_controller)) (Transformation|GetWorldLocation (Variables|Default|GetSlider_Collider)))) (Math|Vector|VectorLength (- (Transformation|GetWorldLocation (Variables|/Game/VirtualRealityBP/Blueprints/BP_MotionController.BP_MotionController_C|GetMotionController _asbp_motion_controller)) (Transformation|GetWorldLocation (Variables|Default|GetSecondHand_Collider)))))
      ;;[0.1333 0.1333 0.1333] Slider Grab
      (Transformation|AttachComponentToComponent AttachToMe (Variables|Default|GetSlider_SM) "" "SnapToTarget" "SnapToTarget" "KeepWorld" true)
      (if (Utilities|Enum|Equal(Enum) (Variables|Default|GetdominantHand) "Left")
        ;;;[0.1094 0.1094 0.1094] Left Hand Dominant
        (Transformation|SetRelativeRotation AttachToMe "0, 0,180.000000" false false)
        (else
          ;;;[0.1094 0.1094 0.1094] Right Hand Dominant
          (Transformation|SetRelativeRotation AttachToMe "0, 0, 0" false false)))
      (Variables|Default|SetSecondHandGrabbed true)
      (bind _output_get (Variables|Default|SetSecond%20Hand%20Motion%20Controller _asbp_motion_controller))
      (Variables|Default|SetSecond%20Hand%20Mesh AttachToMe)
      (Variables|Default|SetX_Last_Position (Math|Vector|MakeVector (.x (Math|Transform|InverseTransformLocation (Transformation|GetWorldTransform (Variables|Default|GetFirearm_SM)) (Transformation|GetWorldLocation (Variables|/Game/VirtualRealityBP/Blueprints/BP_MotionController.BP_MotionController_C|GetMotionController (Variables|Default|GetSecond%20Hand%20Motion%20Controller))))) 0.0 0.0))
      (Variables|/Game/VirtualRealityBP/Blueprints/BP_MotionController.BP_MotionController_C|SetGripState _output_get (Variables|Default|GetLever_Grip_State))
      (Timeline|Timeline_1_0 PlayFromStart
        (:Update
          (if (Utilities|Enum|NotEqual(Enum) (Variables|/Game/VirtualRealityBP/Blueprints/BP_MotionController.BP_MotionController_C|GetGripState (Variables|Default|GetSecond%20Hand%20Motion%20Controller)) "NewEnumerator0")
            (if (Variables|Default|GetSecondHandGrabbed)
              (bind _output_get_2 (Variables|Default|SetX_Delta (- (.x (Math|Transform|InverseTransformLocation (Transformation|GetWorldTransform (Variables|Default|GetFirearm_SM)) (Transformation|GetWorldLocation (Variables|/Game/VirtualRealityBP/Blueprints/BP_MotionController.BP_MotionController_C|GetMotionController (Variables|Default|GetSecond%20Hand%20Motion%20Controller))))) (.x (Variables|Default|GetX_Last_Position)))))
              (Variables|Default|SetX_Last_Position (Math|Vector|MakeVector (+ _output_get_2 (.x (Variables|Default|GetX_Last_Position))) 0.0 0.0))
              (Transformation|AddRelativeLocation _slider_sm (Math|Vector|MakeVector _output_get_2 0.0 0.0) true true)
              (if (> (.x (Variables|/Script/Engine.SceneComponent|GetRelativeLocation _slider_sm)) (Variables|Default|GetSliderXMax))
                (Transformation|SetRelativeLocation _slider_sm "0, 0, 0" false false)
                (elif (< (.x (Variables|/Script/Engine.SceneComponent|GetRelativeLocation _slider_sm)) _sliderxmin)
                  (Transformation|SetRelativeLocation _slider_sm (Math|Vector|MakeVector _sliderxmin 0.0 0.0) false false)))
              (else
                (CallFunction|SliderRevertPosition :!label _label) ; left side  connects from the two branches, right side stops the timeline
                (CallFunction|SecondHandRelease)
                (Timeline|Timeline_1_0 Stop)))
            (else
              (goto _label)))))
      (else
        ;;[0.1329 0.1329 0.1329] Second Hand Guide
        (Variables|Default|SetSecondHandGrabbed true)
        (Transformation|AttachComponentToComponent AttachToMe (Variables|Default|GetFirearm_SM) "Second_Hand_Socket" "SnapToTarget" "SnapToTarget" "KeepWorld" true)
        (if (Utilities|Enum|Equal(Enum) (Variables|Default|GetdominantHand) "Left")
          ;;;[0.1094 0.1094 0.1094] Left Hand Dominant
          (Transformation|SetRelativeRotation AttachToMe "0, 0,180.000000" false false)
          (else
            ;;;[0.1094 0.1094 0.1094] Right Hand Dominant
            (Transformation|SetRelativeRotation AttachToMe "0, 0, 0" false false)))
        (bind _output_get_3 (Variables|Default|SetSecond%20Hand%20Motion%20Controller _asbp_motion_controller))
        (Variables|/Game/VirtualRealityBP/Blueprints/BP_MotionController.BP_MotionController_C|SetGripState _output_get_3 (Variables|Default|GetSecondary_Grip_State))
        (Variables|Default|SetSecond%20Hand%20Mesh AttachToMe)
        (Timeline|Timeline_2 Play
          (:Update
            (if (Utilities|Enum|NotEqual(Enum) (Variables|/Game/VirtualRealityBP/Blueprints/BP_MotionController.BP_MotionController_C|GetGripState (Variables|Default|GetSecond%20Hand%20Motion%20Controller)) "NewEnumerator0")
              (if (Variables|Default|GetSecondHandGrabbed)
                (if (Utilities|Enum|Equal(Enum) (Variables|Default|GetdominantHand) "Left")
                  ;;;[0.4118 0.4118 0.4118] Left Hand Dominant
                  (Transformation|SetRelativeRotation _firearm_sm (Math|Rotator|MakeRotator 0.0 _recoilactual 0.0) false false)
                  (else
                    ;;;[0.4118 0.4118 0.4118] Right Hand Dominant
                    (Transformation|SetRelativeRotation _firearm_sm (Math|Rotator|MakeRotator 1.8e+02 _recoilactual 0.0) false false)))
                (else
                  (CallFunction|SecondHandRelease :!label _label_2)
                  (Timeline|Timeline_2 Stop)))
              (else
                (goto _label_2)))))))
    (else
      ;;[0.1771 0.1771 0.1771] First Hand Grabbed
      (if (Variables|Default|GetOnMagnetMount)
        (Variables|/Game/Blueprints/Tools/BP_MagneticPlacement.BP_MagneticPlacement_C|SetOccupied (Variables|Default|GetMagnetMount) false)
        (Variables|Default|SetOnMagnetMount false))
      (Default|Grab (Variables|Default|GetGrabbableObjectSocket) (Variables|Default|GetFirearm_SM) self HandSocket AttachToMe)
      (bind _aspawn (Utilities|Casting|CastToPawn (Components|GetOwner (Components|GetOwner AttachToMe))))
      (Variables|Default|SetGunOwner _aspawn)
      (Variables|Default|SetFirstHandGrabbed true)
      (Variables|Default|SetSecondHandGrabbed false)
      (Variables|Default|SetFirst%20Hand AttachToMe)
      (bind _asbp_motion_controller_2 (Utilities|Casting|CastToBP_MotionController Actor))
      (Variables|Default|SetdominantHand (Variables|/Game/VirtualRealityBP/Blueprints/BP_MotionController.BP_MotionController_C|GetHand _asbp_motion_controller_2))
      (Variables|/Game/VirtualRealityBP/Blueprints/BP_MotionController.BP_MotionController_C|SetGripState _asbp_motion_controller_2 (Variables|Default|GetPrimary_Grip_State)))))

(fn ConstructionScript
  (|CallParentFunction))