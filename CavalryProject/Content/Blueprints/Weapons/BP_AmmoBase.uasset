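; Base Blueprint for motion-controller grabbable ammo (magazines or shells), with capacity set from ammo type in the Construction Script.
; A GrabbableObjectSocket component handles grab and release; releasing snaps it into an overlapping, unloaded, compatible firearm's magazine port and calls Reload.
; Otherwise, it attaches to the closest free, type-compatible BP_MagneticPlacement mount, tracked through overlap events.
; An attached display actor shows remaining shots, but its show/hide calls are disconnected.
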(event OnComponentBeginOverlap(MagnetCollision)
  (params (OverlappedComponent :type Primitive%20Component%20Object%20Reference) (OtherActor :type Actor%20Object%20Reference) (OtherComp :type Primitive%20Component%20Object%20Reference) (OtherBodyIndex :type Integer) (bFromSweep :type Boolean) (SweepResult :type Hit%20Result%20Structure%20%28by%20ref%29))
  ;[0 0 0] Magnetic
  (bind _asbp_magnetic_placement (Utilities|Casting|CastToBP_MagneticPlacement OtherActor))
  (Utilities|Array|Add (Variables|Default|GetOverlappingMagnets) _asbp_magnetic_placement))

(event OnComponentEndOverlap(MagnetCollision)
  (params (OverlappedComponent :type Primitive%20Component%20Object%20Reference) (OtherActor :type Actor%20Object%20Reference) (OtherComp :type Primitive%20Component%20Object%20Reference) (OtherBodyIndex :type Integer))
  ;[0 0 0] Magnetic
  (bind _asbp_magnetic_placement (Utilities|Casting|CastToBP_MagneticPlacement OtherActor))
  (Utilities|Array|RemoveItem (Variables|Default|GetOverlappingMagnets) _asbp_magnetic_placement))

(event Custom|SnapEvent
  ;[0 0 0] SnapEvent
  (bind _array_element (Utilities|Array|ForEachLoopwithBreak (Collision|GetOverlappingActors (Variables|Default|GetAmmo_SM) "/Game/Blueprints/Weapons/BP_Firearm_Base.BP_Firearm_Base_C" :!class /Script/Engine.PrimitiveComponent) :!label _label)
    (:LoopBody
      (bind _asbp_firearm_base (Utilities|Casting|CastToBP_Firearm_Base _array_element))
      (if (not (Variables|/Game/Blueprints/Weapons/BP_Firearm_Base.BP_Firearm_Base_C|GetisLoaded _asbp_firearm_base))
        (if (Utilities|Enum|Equal(Enum) (Variables|/Game/Blueprints/Weapons/BP_Firearm_Base.BP_Firearm_Base_C|GetloadType _asbp_firearm_base) (Variables|Default|GetAmmoType))
          (Transformation|AttachActorToActor (Components|GetOwner (Variables|Default|GetAmmo_SM)) _asbp_firearm_base "Magazine_Port" "SnapToTarget" "SnapToTarget" "SnapToTarget" true)
          (Variables|Default|SetInGun true)
          (Collision|SetCollisionEnabled (Variables|Default|GetAmmo_SM) "NoCollision")
          (Collision|SetCollisionEnabled (Variables|Default|GetMagnetCollision) "NoCollision")
          (Default|Reload _asbp_firearm_base self (Variables|Default|GetMagazineAmmo))
          (goto _label Break))))))

(event Custom|OnAmmoChange
  (params (RemainingShots :type Integer))
  (Default|UpdateAmmo (Variables|Default|GetAmmoWidget_Ref) RemainingShots))

(event Custom|Ammo_Grab_Audio
  ;[1 0 1] Ammo Audio
)

(event EventBeginPlay
  (bind _returnvalue (Game|SpawnActorfromClass "/Game/HUD/Widgets/Ammo_Display/AmmoDisplay.AmmoDisplay_C" (Math|Transform|MakeTransform "0, 0, 0") "AdjustIfPossibleButAlwaysSpawn" self 0))
  (bind _output_get (Variables|Default|SetAmmoWidget_Ref _returnvalue))
  (Transformation|AttachComponentToComponent _output_get (Variables|Default|GetAmmoWidget_SpawnLoc) "None" "KeepRelative" "KeepRelative" "KeepRelative" false)
  (CallFunction|OnAmmoChange (Variables|Default|GetMagazineAmmo)))

(event EventRelease
  (params (NewParam :type EControllerHand%20Enum :default "Left"))
  ;[0 0 0] Releasing
  (Default|Release (Variables|Default|GetGrabbableObjectSocket))
  (Variables|Default|SetIsGrabbed false)
  (CallFunction|SnapEvent)
  (if (== (Utilities|Array|Length (Variables|Default|GetOverlappingMagnets)) 0)
    (Variables|/Game/VirtualRealityBP/Blueprints/BP_MotionController.BP_MotionController_C|SetGripState (Variables|Default|GetAs%20BP%20Motion%20Controller) "NewEnumerator0")
    (else
      (CallFunction|Magnetize (Utilities|Array|Get(acopy) (Variables|Default|GetOverlappingMagnets))))))

(event EventGrab
  (params (HandSocket :type Name :default "None") (AttachToMe :type Scene%20Component%20Object%20Reference) (Actor :type Actor%20Object%20Reference))
  ;[0 0 0] Grabbing
  (Default|Grab (Variables|Default|GetGrabbableObjectSocket) (Variables|Default|GetAmmo_SM) self "Hand_Magazine_Socket" AttachToMe)
  (CallFunction|AmmoGrabAudio)
  (Variables|Default|SetIsGrabbed true)
  (bind _asbp_motion_controller (Utilities|Casting|CastToBP_MotionController Actor))
  (bind _output_get (Variables|Default|SetAs%20BP%20Motion%20Controller _asbp_motion_controller))
  (Variables|/Game/VirtualRealityBP/Blueprints/BP_MotionController.BP_MotionController_C|SetGripState _output_get (Variables|Default|GetGrip%20State))
  (if (Variables|Default|GetOnMagnetMount)
    (Variables|/Game/Blueprints/Tools/BP_MagneticPlacement.BP_MagneticPlacement_C|SetOccupied (Variables|Default|GetMagnetMount) false)
    (Variables|Default|SetOnMagnetMount false)))

(event EventMagnetize
  (params (Magnet :type Actor%20Object%20Reference))
  (bind _ammo_sm (Variables|Default|GetAmmo_SM))
  (bind _magnetcollision (Variables|Default|GetMagnetCollision))
  (bind _returnvalue (Transformation|GetWorldLocation _magnetcollision))
  ;[0 0 0] Magnetic
  (if (not (Variables|Default|GetInGun))
    (if (not (Variables|Default|GetIsGrabbed))
      (Variables|Default|SetClosestMount 0)
      (for _array_element (Variables|Default|GetOverlappingMagnets)
        (if (not (Variables|/Game/Blueprints/Tools/BP_MagneticPlacement.BP_MagneticPlacement_C|GetOccupied _array_element))
          (if (or (Utilities|Enum|Equal(Enum) (Variables|Default|GetAmmo%20Object%20Type) (Variables|/Game/Blueprints/Tools/BP_MagneticPlacement.BP_MagneticPlacement_C|GetObject%20Type _array_element)) (Utilities|Enum|Equal(Enum) (Variables|/Game/Blueprints/Tools/BP_MagneticPlacement.BP_MagneticPlacement_C|GetObject%20Type _array_element) "NewEnumerator0"))
            (if (Utilities|IsValid (Variables|Default|GetClosestMount))
              (if (< (Math|Vector|VectorLength (- _returnvalue (Transformation|GetWorldLocation (Variables|/Script/Engine.Actor|GetRootComponent _array_element)))) (Math|Vector|VectorLength (- _returnvalue (Transformation|GetWorldLocation (Variables|/Script/Engine.Actor|GetRootComponent (Variables|Default|GetClosestMount))))))
                (Variables|Default|SetClosestMount _array_element))
              (else
                (Variables|Default|SetClosestMount _array_element))))))
      (if (Utilities|IsValid (Variables|Default|GetClosestMount))
        (Physics|SetSimulatePhysics _ammo_sm false)
        (Transformation|AttachComponentToComponent _ammo_sm (Variables|/Script/Engine.Actor|GetRootComponent (Variables|Default|GetClosestMount)) "None" "SnapToTarget" "SnapToTarget" "KeepWorld" false)
        (Variables|Default|SetOnMagnetMount true)
        (bind _output_get (Variables|Default|SetMagnetMount (Variables|Default|GetClosestMount)))
        (Variables|/Game/Blueprints/Tools/BP_MagneticPlacement.BP_MagneticPlacement_C|SetOccupied _output_get true)))))

(fn ConstructionScript
  (switch Utilities|FlowControl|Switch|SwitchonE_LoadType (Variables|Default|GetAmmoType)
    (:NewEnumerator0
      (Variables|Default|SetMagazineAmmo 12))
    (:NewEnumerator2
      (Variables|Default|SetMagazineAmmo 30 :!label _label))
    (:NewEnumerator3
      (Variables|Default|SetMagazineAmmo 20))
    (:NewEnumerator4
      (goto _label))
    (:NewEnumerator1
      (Variables|Default|SetMagazineAmmo 1))))