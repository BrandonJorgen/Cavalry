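; Shotgun shell ammo, a child of an ammo base Blueprint, that snaps into a firearm to load it.
; SnapEvent finds an overlapping firearm with a matching load type and a current ammo count within a hardcoded limit.
; It attaches the shell to the gun's magazine port socket, disables mesh and magnet collision, then calls the firearm's Reload with itself and its magazine ammo.
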(event EventSnapEvent
  ;[0 0 0] SnapEvent
  (bind _array_element (Utilities|Array|ForEachLoopwithBreak (Collision|GetOverlappingActors (Variables|Default|GetAmmo_SM) "/Game/Blueprints/Weapons/BP_Firearm_Base.BP_Firearm_Base_C" :!class /Script/Engine.PrimitiveComponent) :!label _label)
    (:LoopBody
      (bind _asbp_firearm_base (Utilities|Casting|CastToBP_Firearm_Base _array_element))
      (if (not (> (Variables|/Game/Blueprints/Weapons/BP_Firearm_Base.BP_Firearm_Base_C|GetcurrentAmmo _asbp_firearm_base) 7))
        (if (Utilities|Enum|Equal(Enum) (Variables|/Game/Blueprints/Weapons/BP_Firearm_Base.BP_Firearm_Base_C|GetloadType _asbp_firearm_base) (Variables|Default|GetAmmoType))
          (Transformation|AttachActorToActor (Components|GetOwner (Variables|Default|GetAmmo_SM)) _asbp_firearm_base "Magazine_Port" "SnapToTarget" "SnapToTarget" "SnapToTarget" true)
          (Variables|Default|SetInGun true)
          (Collision|SetCollisionEnabled (Variables|Default|GetAmmo_SM) "NoCollision")
          (Collision|SetCollisionEnabled (Variables|Default|GetMagnetCollision) "NoCollision")
          (Default|Reload _asbp_firearm_base self (Variables|Default|GetMagazineAmmo))
          (goto _label Break))))))

(fn ConstructionScript
  (|CallParentFunction))