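; Base VR melee weapon (knife) that motion controllers grab, use to damage enemies or destructibles, and stow on magnetic mounts.
; Grab attaches the mesh to the hand socket, using a dot product against the hand to decide whether to flip the blade.
; Damage-trigger overlaps line trace the struck component, scaling enemy damage by bone and doubling it for out-of-combat targets.
; Release disables damage and snaps the weapon to the closest free, type-compatible overlapping mount.
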(event OnComponentBeginOverlap(MagnetCollision)
  (params (OverlappedComponent :type Primitive%20Component%20Object%20Reference) (OtherActor :type Actor%20Object%20Reference) (OtherComp :type Primitive%20Component%20Object%20Reference) (OtherBodyIndex :type Integer) (bFromSweep :type Boolean) (SweepResult :type Hit%20Result%20Structure%20%28by%20ref%29))
  ;[0 0 0] Magnetic
  (bind _asbp_magnetic_placement (Utilities|Casting|CastToBP_MagneticPlacement OtherActor))
  (Utilities|Array|Add (Variables|Mount|GetOverlappingMagnets) _asbp_magnetic_placement))

(event OnComponentBeginOverlap(DamageTrigger)
  (params (OverlappedComponent :type Primitive%20Component%20Object%20Reference) (OtherActor :type Actor%20Object%20Reference) (OtherComp :type Primitive%20Component%20Object%20Reference) (OtherBodyIndex :type Integer) (bFromSweep :type Boolean) (SweepResult :type Hit%20Result%20Structure%20%28by%20ref%29))
  ;[0 0 0] Damage
  (bind (_hitlocation _hitnormal _bonename _outhit) (Collision|LineTraceComponent OtherComp (Transformation|GetWorldLocation (Variables|Default|GetMelee_SM)) (Transformation|GetWorldLocation (Variables|Default|GetTraceEnd)) true false false))
  (switch Utilities|FlowControl|Switch|SwitchonECollisionChannel (Collision|GetCollisionObjectType (.hitcomponent _outhit))
    (:ECC_Destructible
      (Class|BPIShootable|Shot(Message) (.hitactor _outhit)))
    (:ECC_GameTraceChannel1
      (bind _asbp_enemy_base (Utilities|Casting|CastToBP_EnemyBase OtherActor))
      (bind _asaic_enemy (Utilities|Casting|CastToAIC_Enemy (AI|GetAIController _asbp_enemy_base)))
      (Variables|Attack|SetTargetInCombat (Variables|/Game/Blueprints/Enemies/AIC_Enemy.AIC_Enemy_C|GetInCombat _asaic_enemy))
      (Utilities|BoneNameDamageCalc _bonename
        (:Exit
          (Class|BPITakeDamage|TakeDamageActor(Message) OtherActor (Variables|Attack|GetDamageAmount) (Variables|Base|GetKnifeOwner))
          (Default|RumbleController (Variables|Base|GetGrabbing%20Hand) 0.2)
          ;[1 0 1] Knife Hit Audio
          (CallFunction|KnifeHitAudio))))))

(event OnComponentEndOverlap(MagnetCollision)
  (params (OverlappedComponent :type Primitive%20Component%20Object%20Reference) (OtherActor :type Actor%20Object%20Reference) (OtherComp :type Primitive%20Component%20Object%20Reference) (OtherBodyIndex :type Integer))
  ;[0 0 0] Magnetic
  (bind _asbp_magnetic_placement (Utilities|Casting|CastToBP_MagneticPlacement OtherActor))
  (Utilities|Array|RemoveItem (Variables|Mount|GetOverlappingMagnets) _asbp_magnetic_placement))

(event Custom|Knife_Hit_Audio
  ;[1 0 1] Knife Audio
  (Audio|PlaySoundatLocation "/Game/SFX/Placeholder_SFX/Knife_Placeholders/Knife_Hit_PH.Knife_Hit_PH" (Transformation|GetActorLocation) "0, 0, 0" 1.0 1.0 0.0 0 0 0))

(event Custom|Knife_Grab_Audio
  ;[1 0 1] Knife Audio
)

(event EventMagnetize
  (params (Magnet :type Actor%20Object%20Reference))
  (bind _melee_sm (Variables|Default|GetMelee_SM))
  (bind _magnetcollision (Variables|Default|GetMagnetCollision))
  (bind _returnvalue (Transformation|GetWorldLocation _magnetcollision))
  ;[0 0 0] Magnetic
  (if (not (Variables|Base|GetIsGrabbed))
    (Variables|Mount|SetClosestMount 0)
    (for _array_element (Variables|Mount|GetOverlappingMagnets)
      (if (not (Variables|/Game/Blueprints/Tools/BP_MagneticPlacement.BP_MagneticPlacement_C|GetOccupied _array_element))
        (if (or (Utilities|Enum|Equal(Enum) (Variables|Mount|GetWeaponObjectType) (Variables|/Game/Blueprints/Tools/BP_MagneticPlacement.BP_MagneticPlacement_C|GetObject%20Type _array_element)) (Utilities|Enum|Equal(Enum) (Variables|/Game/Blueprints/Tools/BP_MagneticPlacement.BP_MagneticPlacement_C|GetObject%20Type _array_element) "NewEnumerator0"))
          (if (Utilities|IsValid (Variables|Mount|GetClosestMount))
            (if (< (Math|Vector|VectorLength (- _returnvalue (Transformation|GetWorldLocation (Variables|/Script/Engine.Actor|GetRootComponent _array_element)))) (Math|Vector|VectorLength (- _returnvalue (Transformation|GetWorldLocation (Variables|/Script/Engine.Actor|GetRootComponent (Variables|Mount|GetClosestMount))))))
              (Variables|Mount|SetClosestMount _array_element))
            (else
              (Variables|Mount|SetClosestMount _array_element))))))
    (if (Utilities|IsValid (Variables|Mount|GetClosestMount))
      (Physics|SetSimulatePhysics _melee_sm false)
      (Transformation|AttachComponentToComponent _melee_sm (Variables|/Script/Engine.Actor|GetRootComponent (Variables|Mount|GetClosestMount)) "None" "SnapToTarget" "SnapToTarget" "KeepWorld" false)
      (Variables|Mount|SetOnMagnetMount true)
      (bind _output_get (Variables|Mount|SetMagnetMount (Variables|Mount|GetClosestMount)))
      (Variables|/Game/Blueprints/Tools/BP_MagneticPlacement.BP_MagneticPlacement_C|SetOccupied _output_get true))))

(event EventGrab
  (params (HandSocket :type Name :default "None") (AttachToMe :type Scene%20Component%20Object%20Reference) (Actor :type Actor%20Object%20Reference))
  (bind _asbp_motion_controller (Utilities|Casting|CastToBP_MotionController (Components|GetOwner AttachToMe)))
  (Variables|Base|SetGrabbing%20Hand _asbp_motion_controller)
  (Utilities|IsValid (Variables|Mount|GetMagnetMount)
    (:Is%20Valid
      (if (not (== (Actor|GetAttachParentActor (Variables|Mount|GetMagnetMount)) _asbp_motion_controller))
        ;[0 0 0] Determines if the knfie should be blade up or down in the player's hand
        (if (> (Math|Vector|DotProduct (Math|Vector|GetRightVector (Variables|/Game/VirtualRealityBP/Blueprints/BP_MotionController.BP_MotionController_C|GetHandMesh _asbp_motion_controller)) (Math|Vector|GetUpVector (Variables|Default|GetMelee_SM))) 0.0) :!label _label
          (Default|Grab (Variables|Default|GetGrabbableObjectSocket) (Variables|Default|GetMelee_SM) self HandSocket AttachToMe)
          (Collision|SetCollisionEnabled (Variables|Default|GetDamageTrigger) "QueryAndPhysics")
          (bind _aspawn (Utilities|Casting|CastToPawn (Components|GetOwner (Components|GetOwner AttachToMe))))
          (Variables|Base|SetKnifeOwner _aspawn)
          (else
            (Default|Grab (Variables|Default|GetGrabbableObjectSocket) (Variables|Default|GetMelee_SM) self HandSocket AttachToMe)
            (Collision|SetCollisionEnabled (Variables|Default|GetDamageTrigger) "QueryOnly")
            (bind _aspawn_2 (Utilities|Casting|CastToPawn (Components|GetOwner (Components|GetOwner AttachToMe))))
            (Variables|Base|SetKnifeOwner _aspawn_2)
            (Transformation|AddRelativeRotation (Variables|Default|GetMelee_SM) "0, 0,180.000000" false false)))
        (Variables|Base|SetIsGrabbed true)
        (Variables|/Game/VirtualRealityBP/Blueprints/BP_MotionController.BP_MotionController_C|SetGripState _asbp_motion_controller "NewEnumerator19")
        (if (Variables|Mount|GetOnMagnetMount)
          (Variables|/Game/Blueprints/Tools/BP_MagneticPlacement.BP_MagneticPlacement_C|SetOccupied (Variables|Mount|GetMagnetMount) false)
          (Variables|Mount|SetOnMagnetMount false)
          (Variables|Mount|SetMagnetMount 0)
          (CallFunction|KnifeGrabAudio))))
    (:Is%20Not%20Valid
      (goto _label))))

(event EventRelease
  (params (NewParam :type EControllerHand%20Enum :default "Left"))
  (Default|Release (Variables|Default|GetGrabbableObjectSocket))
  (Collision|SetCollisionEnabled (Variables|Default|GetDamageTrigger) "NoCollision")
  (Variables|Base|SetIsGrabbed false)
  (CallFunction|Magnetize))

(fn ConstructionScript)