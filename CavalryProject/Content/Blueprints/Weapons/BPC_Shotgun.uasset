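; VR shotgun Blueprint that handles two-handed gripping and pump-slider movement with motion controllers.
; The first grab attaches the firearm and sets the dominant hand; the second snaps that hand to the slider.
; A timeline then aims the gun at the second controller with hand-specific roll and recoil pitch.
; While the gun cannot fire, controller movement in gun-local X drives the slider within its limits.
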(event EventSliderRevertPosition
  ;[0 0 0] Slider Reset
  (Variables|Default|SetSecondHandGrabbed false))

(event EventGrab
  (params (HandSocket :type Name :default "None") (AttachToMe :type Scene%20Component%20Object%20Reference) (Actor :type Actor%20Object%20Reference))
  (bind _recoilactual (Variables|Default|GetRecoilActual))
  (bind _sliderxmin (Variables|Default|GetSliderXMin))
  (bind _slider_sm (Variables|Default|GetSlider_SM))
  (bind _firearm_sm (Variables|Default|GetFirearm_SM))
  (bind _firearm_sm_2 (Variables|Default|GetFirearm_SM))
  (bind _firearm_sm_3 (Variables|Default|GetFirearm_SM))
  (bind _firearm_sm_4 (Variables|Default|GetFirearm_SM))
  (bind _relativerotation (Variables|/Script/Engine.SceneComponent|GetRelativeRotation _firearm_sm_4))
  (bind _returnvalue (+ (.pitch _relativerotation) _recoilactual))
  ;[0 0 0] Grabbing
  (if (Variables|Default|GetFirstHandGrabbed)
    ;;[0.1333 0.1333 0.1333] Slider Grab
    (Variables|Default|SetSecondHandGrabbed true)
    (Transformation|AttachComponentToComponent AttachToMe (Variables|Default|GetSlider_SM) "" "SnapToTarget" "SnapToTarget" "KeepWorld" true)
    (if (Utilities|Enum|Equal(Enum) (Variables|Default|GetdominantHand) "Left")
      ;;;[0.1094 0.1094 0.1094] Left Hand Dominant
      (Transformation|SetRelativeRotation AttachToMe "0.000000, 0,180.000000" false false)
      (else
        ;;;[0.1094 0.1094 0.1094] Right Hand Dominant
        (Transformation|SetRelativeRotation AttachToMe "0, 0, 0" false false)))
    (bind _asbp_motion_controller (Utilities|Casting|CastToBP_MotionController Actor))
    (bind _output_get (Variables|Default|SetSecond%20Hand%20Motion%20Controller _asbp_motion_controller))
    (Variables|Default|SetSecond%20Hand%20Mesh AttachToMe)
    (Variables|Default|SetX_Last_Position (Math|Vector|MakeVector (.x (Math|Transform|InverseTransformLocation (Transformation|GetWorldTransform (Variables|Default|GetFirearm_SM)) (Transformation|GetWorldLocation (Variables|/Game/VirtualRealityBP/Blueprints/BP_MotionController.BP_MotionController_C|GetMotionController (Variables|Default|GetSecond%20Hand%20Motion%20Controller))))) 0.0 0.0))
    (Variables|Default|SetStarting%20X%20Position (.x (Math|Transform|InverseTransformLocation (Transformation|GetWorldTransform (Variables|Default|GetFirearm_SM)) (Transformation|GetWorldLocation (Variables|/Game/VirtualRealityBP/Blueprints/BP_MotionController.BP_MotionController_C|GetMotionController (Variables|Default|GetSecond%20Hand%20Motion%20Controller))))))
    (Variables|/Game/VirtualRealityBP/Blueprints/BP_MotionController.BP_MotionController_C|SetGripState _output_get (Variables|Default|GetSecondary_Grip_State))
    (Timeline|Timeline_1_0 PlayFromStart
      (:Update
        (if (Utilities|Enum|NotEqual(Enum) (Variables|/Game/VirtualRealityBP/Blueprints/BP_MotionController.BP_MotionController_C|GetGripState (Variables|Default|GetSecond%20Hand%20Motion%20Controller)) "NewEnumerator0")
          (if (Variables|Default|GetSecondHandGrabbed)
            (Transformation|SetWorldRotation _firearm_sm_2 (Math|Rotator|FindLookatRotation (Transformation|GetWorldLocation _firearm_sm) (Transformation|GetWorldLocation (Variables|/Game/VirtualRealityBP/Blueprints/BP_MotionController.BP_MotionController_C|GetMotionController (Variables|Default|GetSecond%20Hand%20Motion%20Controller)))) false false)
            (if (Utilities|Enum|Equal(Enum) (Variables|Default|GetdominantHand) "Left")
              ;;;[0.3438 0.3438 0.3438] Left Hand Dominant
              (Transformation|SetRelativeRotation _firearm_sm_3 (Math|Rotator|MakeRotator 0.0 _returnvalue (.yaw _relativerotation)) false false)
              (else
                ;;;[0.3438 0.3438 0.3438] Right Hand Dominant
                (Transformation|SetRelativeRotation _firearm_sm_3 (Math|Rotator|MakeRotator 1.8e+02 _returnvalue (.yaw _relativerotation)) false false)))
            (if (Variables|Default|GetcanFire)
              (Transformation|SetRelativeLocation _firearm_sm_2 "0, 0, 0" false false)
              (elif (and (< (.x (Math|Transform|InverseTransformLocation (Transformation|GetWorldTransform _firearm_sm) (Transformation|GetWorldLocation (Variables|/Game/VirtualRealityBP/Blueprints/BP_MotionController.BP_MotionController_C|GetMotionController (Variables|Default|GetSecond%20Hand%20Motion%20Controller))))) (Variables|Default|GetStarting%20X%20Position)) (> (.x (Math|Transform|InverseTransformLocation (Transformation|GetWorldTransform _firearm_sm) (Transformation|GetWorldLocation (Variables|/Game/VirtualRealityBP/Blueprints/BP_MotionController.BP_MotionController_C|GetMotionController (Variables|Default|GetSecond%20Hand%20Motion%20Controller))))) (Variables|Default|GetSliderXMin)))
                (bind _output_get_2 (Variables|Default|SetX_Delta (- (.x (Math|Transform|InverseTransformLocation (Transformation|GetWorldTransform _firearm_sm) (Transformation|GetWorldLocation (Variables|/Game/VirtualRealityBP/Blueprints/BP_MotionController.BP_MotionController_C|GetMotionController (Variables|Default|GetSecond%20Hand%20Motion%20Controller))))) (.x (Variables|Default|GetX_Last_Position)))))
                (Variables|Default|SetX_Last_Position (Math|Vector|MakeVector (+ _output_get_2 (.x (Variables|Default|GetX_Last_Position))) 0.0 0.0))
                (Transformation|AddRelativeLocation _slider_sm (Math|Vector|MakeVector _output_get_2 0.0 0.0) true true)
                (if (> (.x (Variables|/Script/Engine.SceneComponent|GetRelativeLocation _slider_sm)) (Variables|Default|GetSliderXMax))
                  (Transformation|SetRelativeLocation _slider_sm "0, 0, 0" false false)
                  (elif (< (.x (Variables|/Script/Engine.SceneComponent|GetRelativeLocation _slider_sm)) _sliderxmin)
                    (Transformation|SetRelativeLocation _slider_sm (Math|Vector|MakeVector _sliderxmin 0.0 0.0) false false)))))
            (else
              (CallFunction|SliderRevertPosition :!label _label)
              (CallFunction|SecondHandRelease)
              (Timeline|Timeline_1_0 Stop)))
          (else
            (goto _label)))))
    (else
      ;;[0.1771 0.1771 0.1771] First Hand Grabbed
      (if (Variables|Default|GetOnMagnetMount)
        (Variables|/Game/Blueprints/Tools/BP_MagneticPlacement.BP_MagneticPlacement_C|SetOccupied (Variables|Default|GetMagnetMount) false)
        (Variables|Default|SetOnMagnetMount false))
      (Default|Grab (Variables|Default|GetGrabbableObjectSocket) (Variables|Default|GetFirearm_SM) self HandSocket AttachToMe)
      (bind _aspawn (Utilities|Casting|CastToPawn (Components|GetOwner (Components|GetOwner AttachToMe))))
      (Variables|Default|SetGunOwner _aspawn)
      (Variables|Default|SetFirstHandGrabbed true)
      (Variables|Default|SetSecondHandGrabbed false)
      (Variables|Default|SetFirst%20Hand AttachToMe)
      (bind _asbp_motion_controller_2 (Utilities|Casting|CastToBP_MotionController Actor))
      (Variables|Default|SetdominantHand (Variables|/Game/VirtualRealityBP/Blueprints/BP_MotionController.BP_MotionController_C|GetHand _asbp_motion_controller_2))
      (Variables|/Game/VirtualRealityBP/Blueprints/BP_MotionController.BP_MotionController_C|SetGripState _asbp_motion_controller_2 (Variables|Default|GetPrimary_Grip_State)))))

(fn ConstructionScript
  (|CallParentFunction))