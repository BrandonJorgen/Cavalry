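; Grabbable cicada grenade tool for motion-controller play, which spawns a smoke effect shortly after being armed and released.
; A first grab attaches the grenade to the controller; a grab while held spawns a pin actor into that hand, arms the grenade and plays its active pose.
; Releasing unarmed calls Magnetize, while releasing armed starts a one-shot delay into Explode, which only prints and spawns smoke.
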(event Custom|Explode
  (bind _tool_skm (Variables|Default|GetTool_SkM))
  (bind _returnvalue (Transformation|GetWorldTransform _tool_skm))
  ;[1 0 0] NIAGRA BIDNESS use the arrow as a point of reference for location
  (Development|PrintString "I JUST EXPLODED GRENADE_BP")
  (Niagara|SpawnSystematLocation "/Game/VisualEffects/Niagara/NE_Smoke_System.NE_Smoke_System" (.location _returnvalue) (.rotation _returnvalue) (.scale _returnvalue)))

(event EventGrab
  (params (HandSocket :type Name :default "None") (AttachToMe :type Scene%20Component%20Object%20Reference) (Actor :type Actor%20Object%20Reference))
  ;[1 1 1] Grabbing
  (if (Variables|Default|GetisGrabbed)
    (if (not (Variables|Default|GetPin%20Removed))
      (bind _returnvalue (Game|SpawnActorfromClass "/Game/Blueprints/Tools/BP_CicadaGrenadePin.BP_CicadaGrenadePin_C" (Transformation|GetWorldTransform (Variables|Default|GetTool_SkM)) "Undefined" 0 0))
      (Default|Grab (Variables|/Game/Blueprints/Tools/BP_CicadaGrenadePin.BP_CicadaGrenadePin_C|GetGrabbableObjectSocket _returnvalue) (Variables|/Game/Blueprints/Tools/BP_CicadaGrenadePin.BP_CicadaGrenadePin_C|GetPIN _returnvalue) _returnvalue HandSocket AttachToMe)
      (Variables|Default|SetPin%20Removed true)
      (bind _asbp_motion_controller (Utilities|Casting|CastToBP_MotionController Actor))
      (Variables|/Game/VirtualRealityBP/Blueprints/BP_MotionController.BP_MotionController_C|SetAttachedActor _asbp_motion_controller _returnvalue)
      (CallFunction|ActivateTool true)
      (Components|Animation|PlayAnimation (Variables|Default|GetTool_SkM) "/Game/Meshes/Placeholder/Tools/Grenade/ActivePose.ActivePose" false))
    (else
      (Default|Grab (Variables|Default|GetGrabbableObjectSocket) (Variables|Default|GetTool_SkM) self "None" AttachToMe)
      (Variables|Default|SetisGrabbed true)
      (bind _asbp_motion_controller_2 (Utilities|Casting|CastToBP_MotionController Actor))
      (Variables|Default|SetPrimary%20Hand (Variables|/Game/VirtualRealityBP/Blueprints/BP_MotionController.BP_MotionController_C|GetHand _asbp_motion_controller_2)))))

(event EventRelease
  (params (NewParam :type EControllerHand%20Enum :default "Left"))
  ;[1 1 1] Releasing
  (if (Variables|Default|GettoolActivated)
    (CallFunction|Activate)
    (Default|Release (Variables|Default|GetGrabbableObjectSocket))
    (Variables|Default|SetisGrabbed false)
    (else
      (Default|Release (Variables|Default|GetGrabbableObjectSocket))
      (Variables|Default|SetisGrabbed false)
      (CallFunction|Magnetize))))

(event EventActivateTool
  (params (Active :type Boolean))
  ;[1 1 1] Activate
  (Variables|Default|SettoolActivated Active))

(event EventActivate
  ;[1 1 1] Activate
  (Utilities|FlowControl|DoOnce false
    (:Completed
      (Utilities|FlowControl|Delay 3.0)
      (CallFunction|Explode))))

(fn ConstructionScript
  (|CallParentFunction))