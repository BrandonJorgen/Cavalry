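; Base Blueprint for grabbable tools that the player holds and activates, and that snap onto magnetic placements when let go.
; GrabbableObjectSocket handles grab and release; grabbing records the owner, frees any mount and triggers a one-time tutorial.
; Release and BeginPlay call Magnetize, which attaches an inactive tool to the nearest overlapping, unoccupied, type-compatible BP_MagneticPlacement.
; ActivateTool works only while held, firing Activate and interrupting the tutorial.
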(event OnComponentBeginOverlap(MagnetCollision)
  (params (OverlappedComponent :type Primitive%20Component%20Object%20Reference) (OtherActor :type Actor%20Object%20Reference) (OtherComp :type Primitive%20Component%20Object%20Reference) (OtherBodyIndex :type Integer) (bFromSweep :type Boolean) (SweepResult :type Hit%20Result%20Structure%20%28by%20ref%29))
  ;[0 0 0] Magnetic
  (bind _asbp_magnetic_placement (Utilities|Casting|CastToBP_MagneticPlacement OtherActor))
  (Utilities|Array|Add (Variables|MagMount|GetOverlappingMagnets) _asbp_magnetic_placement))

(event OnComponentEndOverlap(MagnetCollision)
  (params (OverlappedComponent :type Primitive%20Component%20Object%20Reference) (OtherActor :type Actor%20Object%20Reference) (OtherComp :type Primitive%20Component%20Object%20Reference) (OtherBodyIndex :type Integer))
  ;[0 0 0] Magnetic
  (bind _asbp_magnetic_placement (Utilities|Casting|CastToBP_MagneticPlacement OtherActor))
  (Utilities|Array|RemoveItem (Variables|MagMount|GetOverlappingMagnets) _asbp_magnetic_placement))

(event Custom|Magnetize
  (params (Magnet :type Actor%20Object%20Reference))
  (bind _tool_skm (Variables|Default|GetTool_SkM))
  (bind _magnetcollision (Variables|MagMount|GetMagnetCollision))
  (bind _returnvalue (Transformation|GetWorldLocation _magnetcollision))
  ;[0 0 0] Magnetic
  (if (not (Variables|Default|GettoolActivated))
    (if (not (Variables|Default|GetIsGrabbed))
      (Variables|MagMount|SetClosestMount 0)
      (for _array_element (Variables|MagMount|GetOverlappingMagnets)
        (if (not (Variables|/Game/Blueprints/Tools/BP_MagneticPlacement.BP_MagneticPlacement_C|GetOccupied _array_element))
          (if (or (Utilities|Enum|Equal(Enum) (Variables|MagMount|GetTool%20Object%20Type) (Variables|/Game/Blueprints/Tools/BP_MagneticPlacement.BP_MagneticPlacement_C|GetObject%20Type _array_element)) (Utilities|Enum|Equal(Enum) (Variables|/Game/Blueprints/Tools/BP_MagneticPlacement.BP_MagneticPlacement_C|GetObject%20Type _array_element) "NewEnumerator0"))
            (if (Utilities|IsValid (Variables|MagMount|GetClosestMount))
              (if (< (Math|Vector|VectorLength (- _returnvalue (Transformation|GetWorldLocation (Variables|/Script/Engine.Actor|GetRootComponent _array_element)))) (Math|Vector|VectorLength (- _returnvalue (Transformation|GetWorldLocation (Variables|/Script/Engine.Actor|GetRootComponent (Variables|MagMount|GetClosestMount))))))
                (Variables|MagMount|SetClosestMount _array_element))
              (else
                (Variables|MagMount|SetClosestMount _array_element))))))
      (if (Utilities|IsValid (Variables|MagMount|GetClosestMount))
        (Physics|SetSimulatePhysics _tool_skm false)
        (Transformation|AttachComponentToComponent _tool_skm (Variables|/Script/Engine.Actor|GetRootComponent (Variables|MagMount|GetClosestMount)) "None" "SnapToTarget" "SnapToTarget" "KeepWorld" false)
        (Variables|MagMount|SetOnMagnetMount true)
        (bind _output_get (Variables|MagMount|SetMagnetMount (Variables|MagMount|GetClosestMount)))
        (Variables|/Game/Blueprints/Tools/BP_MagneticPlacement.BP_MagneticPlacement_C|SetOccupied _output_get true)
        (Development|PrintString "WE ARE TRYING TO DO THE THING SIR")))))

(event Custom|Activate
  ;[0 0 0] Activates
  (Development|PrintString "BP_TOOLBASE Ativated")
  (CallFunction|ActivateAudio))

(event Custom|ToolTutorial
  (bind _toolowner (Variables|Default|GetToolOwner))
  ;[0 0 0] Tool Tutorial
  (if (not (Variables|/Game/Blueprints/Characters/BP_PlayerCharacter_Base.BP_PlayerCharacter_Base_C|GetHasSeenToolTutorial _toolowner))
    (Class|BPITutorialText|CallToolTutorial(Message) (Variables|/Game/Blueprints/Characters/BP_PlayerCharacter_Base.BP_PlayerCharacter_Base_C|GetWidgetHandler _toolowner))
    (Variables|/Game/Blueprints/Characters/BP_PlayerCharacter_Base.BP_PlayerCharacter_Base_C|SetHasSeenToolTutorial _toolowner true)
    (Development|PrintString "tool tutorial CALLED")))

(event Custom|InterruptToolTutorial
  (bind _toolowner (Variables|Default|GetToolOwner))
  (bind _widgethandler (Variables|/Game/Blueprints/Characters/BP_PlayerCharacter_Base.BP_PlayerCharacter_Base_C|GetWidgetHandler _toolowner))
  ;[0 0 0] Tool Tutorial
  (if (Variables|/Game/HUD/Widgets/Damage_Display/BP_HorsemenHUD.BP_HorsemenHUD_C|GetToolTutorialAnimating _widgethandler)
    (Class|BPITutorialText|InterruptToolTutorial(Message) _widgethandler)))

(event Custom|Activate_Audio
  ;[1 0 1] Tool Audio
)

(event EventGrab
  (params (HandSocket :type Name :default "None") (AttachToMe :type Scene%20Component%20Object%20Reference) (Actor :type Actor%20Object%20Reference))
  ;[0 0 0] Grabbing
  (Default|Grab (Variables|Default|GetGrabbableObjectSocket) (Variables|Default|GetTool_SkM) self HandSocket AttachToMe)
  (Variables|Default|SetisGrabbed true)
  (bind _asbp_player_character_base (Utilities|Casting|CastToBP_PlayerCharacter_Base (Components|GetOwner Actor)))
  (Variables|Default|SetToolOwner _asbp_player_character_base)
  (CallFunction|ToolTutorial)
  (if (Variables|MagMount|GetOnMagnetMount)
    (Variables|/Game/Blueprints/Tools/BP_MagneticPlacement.BP_MagneticPlacement_C|SetOccupied (Variables|MagMount|GetMagnetMount) false)
    (Variables|MagMount|SetOnMagnetMount false)
    (Variables|MagMount|SetMagnetMount 0)))

(event EventRelease
  (params (NewParam :type EControllerHand%20Enum :default "Left"))
  ;[0 0 0] Releasing
  (Default|Release (Variables|Default|GetGrabbableObjectSocket))
  (Variables|Default|SetisGrabbed false)
  (CallFunction|Magnetize))

(event EventBeginPlay
  (Utilities|FlowControl|Delay 0.1)
  (for _array_element (Collision|GetOverlappingActors (Variables|MagMount|GetMagnetCollision) 0 :!class /Script/Engine.PrimitiveComponent)
    (bind _asbp_magnetic_placement (Utilities|Casting|CastToBP_MagneticPlacement _array_element))
    (Utilities|Array|Add (Variables|MagMount|GetOverlappingMagnets) _asbp_magnetic_placement))
  (CallFunction|Magnetize))

(event EventActivateTool
  (params (Active :type Boolean))
  ;[0 0 0] Activates
  (if (Variables|Default|GetisGrabbed)
    (Variables|Default|SettoolActivated Active)
    (CallFunction|Activate)
    (CallFunction|InterruptToolTutorial)))

(fn ConstructionScript)