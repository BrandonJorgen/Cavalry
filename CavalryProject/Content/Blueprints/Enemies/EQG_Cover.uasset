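; EQG_Cover is an Environment Query generator for enemies that supplies nearby actors of a configurable class, named as cover, as query items.
; On generation it clears its cached list, then gathers every actor of the searched class within a radius of the querier.
; Each match is added as a generated actor, and the passed context locations are unused.
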(fn DoItemGeneration
  (params (ContextLocations :type Array%20of%20Vectors))
  (Utilities|Array|Clear (Variables|Default|GetNearbyActors))
  (bind _asactor (Utilities|Casting|CastToActor (Class|EnvQueryGeneratorBlueprintBase|GetQuerier)))
  (bind _outactors (Actor|GetAllActorsOfClass (Variables|Default|GetSearchedActor)))
  (for _array_element _outactors
    (if (<= (Math|Vector|Distance(Vector) (Transformation|GetActorLocation _array_element) (Transformation|GetActorLocation _asactor)) (Variables|Default|GetRadius))
      (Utilities|Array|Add (Variables|Default|GetNearbyActors) _array_element)))
  (for _array_element_2 (Variables|Default|GetNearbyActors)
    (EQS|AddGeneratedActor _array_element_2))
  (return))