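; AI controller for enemies that runs BT_Enemy2 on possess and feeds it a reserved-cover actor and a TargetActor through the blackboard.
; Pawn sensing targets players on sight, or noise instigators while out of combat, then relays the alert to nearby AI via MakeNoise.
; It clears the target when Conquest, War, Famine or Death signals removal.
; Callable events shrink or restore sight radius for darkness and smoke.
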(event OnHearNoise(PawnSensing)
  (params (Instigator :type Pawn%20Object%20Reference) (Location :type Vector%20%28by%20ref%29 :default "0, 0, 0") (Volume :type Float%20%28single-precision%29))
  ;[0 0 0] Enemy Hearing (Player gun shots or other Enemy voices)
  (if (not (Variables|/Game/Blueprints/Enemies/BP_EnemyBase.BP_EnemyBase_C|GetInCombat (Variables|Default|GetEnemyBase)))
    (CallFunction|UpdateTargetKey Instigator)
    (CallFunction|AlertNearby Instigator)
    (bind _asbp_enemy_base (Utilities|Casting|CastToBP_EnemyBase (Variables|Default|GetPossessed%20Pawn)))
    (Default|PlayerSpotted _asbp_enemy_base)))

(event OnSeePawn(PawnSensing)
  (params (Pawn :type Pawn%20Object%20Reference))
  ;[0 0 0] Player Targeting
  ;;[0.08235 0.08235 0.08235] Do we see an Actor with the Tag of Player?
  (Variables|Default|SetPerceivedActor Pawn)
  (if (Actor|ActorHasTag Pawn "Player")
    (CallFunction|UpdateTargetKey (Variables|Default|GetPerceivedActor))
    (Variables|/Game/Blueprints/Enemies/BP_EnemyBase.BP_EnemyBase_C|SetInCombat (Variables|Default|GetEnemyBase) true)
    (CallFunction|AlertNearby (Variables|Default|GetPerceivedActor))
    (bind _asbp_enemy_base (Utilities|Casting|CastToBP_EnemyBase (Variables|Default|GetPossessed%20Pawn)))
    (Default|PlayerSpotted _asbp_enemy_base)))

(event Custom|AlertNearby
  (params (Pawn :type Pawn%20Object%20Reference))
  ;[0 0 0] Alert other AI nearby to the presence of a target
  (Class|Actor|MakeNoise 1.0 Pawn (Transformation|GetActorLocation (Variables|Default|GetPossessed%20Pawn)) 0.0 "None"))

(event Custom|RemoveAsTarget_Famine
  (if (== (Variables|Default|GetPlayerFamine) (AI|Components|Blackboard|GetValueasObject (Variables|Default|GetBlackboard) (Utilities|Name|MakeLiteralName "TargetActor")))
    (AI|Components|Blackboard|ClearValue (Variables|Default|GetBlackboard) (Utilities|Name|MakeLiteralName "TargetActor"))))

(event Custom|LowerSightRadius
  ;[0 0 0] Lower sight when told its in darkness or smoke
  (Variables|/Script/AIModule.PawnSensingComponent|SetSightRadius (Variables|Default|GetPawnSensing) 5e+02)
  (bind _asbp_enemy_base (Utilities|Casting|CastToBP_EnemyBase (Variables|Default|GetPossessed%20Pawn)))
  (Variables|/Game/Blueprints/Enemies/BP_EnemyBase.BP_EnemyBase_C|SetInDarkness _asbp_enemy_base true))

(event Custom|ResetSightRadius
  ;[0 0 0] Reset the sight radius
  (Variables|/Script/AIModule.PawnSensingComponent|SetSightRadius (Variables|Default|GetPawnSensing) 2.5e+03)
  (bind _asbp_enemy_base (Utilities|Casting|CastToBP_EnemyBase (Variables|Default|GetPossessed%20Pawn)))
  (Variables|/Game/Blueprints/Enemies/BP_EnemyBase.BP_EnemyBase_C|SetInDarkness _asbp_enemy_base false))

(event Custom|RemoveAsTarget_Death
  (if (== (Variables|Default|GetPlayerDeath) (AI|Components|Blackboard|GetValueasObject (Variables|Default|GetBlackboard) (Utilities|Name|MakeLiteralName "TargetActor")))
    (AI|Components|Blackboard|ClearValue (Variables|Default|GetBlackboard) (Utilities|Name|MakeLiteralName "TargetActor"))))

(event Custom|RemoveAsTarget_Conquest
  (if (== (Variables|Default|GetPlayerConquest) (AI|Components|Blackboard|GetValueasObject (Variables|Default|GetBlackboard) (Utilities|Name|MakeLiteralName "TargetActor")))
    (AI|Components|Blackboard|ClearValue (Variables|Default|GetBlackboard) (Utilities|Name|MakeLiteralName "TargetActor"))))

(event Custom|RemoveAsTarget_War
  (if (== (Variables|Default|GetPlayerWar) (AI|Components|Blackboard|GetValueasObject (Variables|Default|GetBlackboard) (Utilities|Name|MakeLiteralName "TargetActor")))
    (AI|Components|Blackboard|ClearValue (Variables|Default|GetBlackboard) (Utilities|Name|MakeLiteralName "TargetActor"))))

(event EventPossess
  (params (PossessedPawn :type Pawn%20Object%20Reference))
  ;[0 0 0] Behavior Tree Selection
  (AI|RunBehaviorTree "/Game/Blueprints/Enemies/BT_Enemy2.BT_Enemy2")
  (bind _returnvalue (Actor|GetActorOfClass "/Game/Blueprints/Enemies/BP_ReservedCover.BP_ReservedCover_C"))
  (AI|Components|Blackboard|SetValueasObject (Variables|Default|GetBlackboard) (Utilities|Name|MakeLiteralName "ReservedCoverArray") _returnvalue)
  (bind _output_get (Variables|Default|SetPossessed%20Pawn PossessedPawn))
  (bind _asbp_enemy_base (Utilities|Casting|CastToBP_EnemyBase _output_get))
  (Variables|Default|SetEnemyBase _asbp_enemy_base)
  (bind _returnvalue_2 (Actor|GetActorOfClass "/Game/Blueprints/Characters/BPC_Conquest.BPC_Conquest_C"))
  (Utilities|IsValid _returnvalue_2
    (:Is%20Valid
      (bind _output_get_2 (Variables|Default|SetPlayerConquest _returnvalue_2))
      (EventDispatchers|AssignRemoveasTarget _output_get_2 (delegate Custom|RemoveAsTarget_Conquest)))
    (:Is%20Not%20Valid
      _))
  (bind _returnvalue_3 (Actor|GetActorOfClass "/Game/Blueprints/Characters/BPC_War.BPC_War_C"))
  (Utilities|IsValid _returnvalue_3
    (:Is%20Valid
      (bind _output_get_3 (Variables|Default|SetPlayerWar _returnvalue_3))
      (EventDispatchers|AssignRemoveasTarget _output_get_3 (delegate Custom|RemoveAsTarget_War)))
    (:Is%20Not%20Valid
      _))
  (bind _returnvalue_4 (Actor|GetActorOfClass "/Game/Blueprints/Characters/BPC_Famine.BPC_Famine_C"))
  (Utilities|IsValid _returnvalue_4
    (:Is%20Valid
      (bind _output_get_4 (Variables|Default|SetPlayerFamine _returnvalue_4))
      (EventDispatchers|AssignRemoveasTarget _output_get_4 (delegate Custom|RemoveAsTarget_Famine)))
    (:Is%20Not%20Valid
      _))
  (bind _returnvalue_5 (Actor|GetActorOfClass "/Game/Blueprints/Characters/BPC_Death.BPC_Death_C"))
  (Utilities|IsValid _returnvalue_5
    (:Is%20Valid
      (bind _output_get_5 (Variables|Default|SetPlayerDeath _returnvalue_5))
      (EventDispatchers|AssignRemoveasTarget _output_get_5 (delegate Custom|RemoveAsTarget_Death)))))

(fn ConstructionScript)

(fn UpdateTargetKey
  (params (Actor :type Actor%20Object%20Reference))
  (Variables|/Game/Blueprints/Enemies/BP_EnemyBase.BP_EnemyBase_C|SetInCombat (Variables|Default|GetEnemyBase) true)
  (AI|Components|Blackboard|SetValueasObject (Variables|Default|GetBlackboard) (Utilities|Name|MakeLiteralName "TargetActor") Actor))

(fn Alert
  (params (TargetActor :type Actor%20Object%20Reference))
  (AI|Components|Blackboard|SetValueasObject (Variables|Default|GetBlackboard) (Utilities|Name|MakeLiteralName "TargetActor") TargetActor))