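; EQS context that supplies the closest player character to the querier, for use in enemy environment queries.
; ProvideSingleActor gets all BP_PlayerCharacter_Base actors and compares each one's distance to the querier against ClosestPlayerDist.
; It stores any nearer distance and actor as it loops, then returns ClosestPlayer as the context actor.
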(fn ProvideSingleActor
  (params (QuerierObject :type Object%20Object%20Reference) (QuerierActor :type Actor%20Object%20Reference))
  (bind _outactors (Actor|GetAllActorsOfClass "/Game/Blueprints/Characters/BP_PlayerCharacter_Base.BP_PlayerCharacter_Base_C"))
  (for _array_element _outactors
    (if (< (Math|Vector|Distance(Vector) (Transformation|GetActorLocation QuerierActor) (Transformation|GetActorLocation _array_element)) (LocalVariables|GetClosestPlayerDist))
      (LocalVariables|SetClosestPlayerDist (Math|Vector|Distance(Vector) (Transformation|GetActorLocation QuerierActor) (Transformation|GetActorLocation _array_element)))
      (LocalVariables|SetClosestPlayer _array_element)))
  (return (LocalVariables|GetClosestPlayer)))