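; Base enemy character that spawns an attached rifle, takes damage, and attacks by shooting or stabbing.
; Server-authoritative damage sets the blackboard death flag or retargets the AI and alerts nearby enemies, updating combat state through GS_Cavalry.
; Shots roll random hits, less likely in darkness; landed attacks trigger the player's damage-direction widget.
; Ground trigger boxes gate on animation state and trace surface type for FMOD footsteps, alongside fire and hurt audio.
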(event OnComponentBeginOverlap(GroundDetectionBox)
  (params (OverlappedComponent :type Primitive%20Component%20Object%20Reference) (OtherActor :type Actor%20Object%20Reference) (OtherComp :type Primitive%20Component%20Object%20Reference) (OtherBodyIndex :type Integer) (bFromSweep :type Boolean) (SweepResult :type Hit%20Result%20Structure%20%28by%20ref%29))
  (bind _returnvalue (Transformation|GetWorldLocation OverlappedComponent))
  ;[0 0 0] Foot Audio TriggerBox
  (Utilities|FlowControl|DoOnce true
    (:Completed
      (bind _asabp_enemy_final (Utilities|Casting|CastToABP_Enemy_Final (Components|SkeletalMesh|GetAnimInstance (Variables|Character|GetMesh))))
      (bind _output_get (Variables|Default|SetEnumState (Variables|/Game/Meshes/Final/Enemy_Mesh/ABP_Enemy_Final.ABP_Enemy_Final_C|GetEnum_State _asabp_enemy_final)))
      (switch Utilities|FlowControl|Switch|SwitchonE_Enemy_Animation_State_Final _output_get
        (:NewEnumerator8
          _)
        (:NewEnumerator2
          _))
      (bind _outhit (Collision|LineTraceForObjects _returnvalue (- _returnvalue "0, 0,10.000000") (Utilities|Array|MakeArray "ObjectTypeQuery1" "ObjectTypeQuery2") false 0 "ForDuration"))
      (CallFunction|EnemyFootstepAudio (Variables|/Script/PhysicsCore.PhysicalMaterial|GetSurfaceType (.physmat _outhit))))))

(event OnComponentBeginOverlap(GroundDetectionBox1)
  (params (OverlappedComponent :type Primitive%20Component%20Object%20Reference) (OtherActor :type Actor%20Object%20Reference) (OtherComp :type Primitive%20Component%20Object%20Reference) (OtherBodyIndex :type Integer) (bFromSweep :type Boolean) (SweepResult :type Hit%20Result%20Structure%20%28by%20ref%29))
  (bind _returnvalue (Transformation|GetWorldLocation OverlappedComponent))
  ;[0 0 0] Foot Audio TriggerBox
  (Utilities|FlowControl|DoOnce true
    (:Completed
      (bind _asabp_enemy_final (Utilities|Casting|CastToABP_Enemy_Final (Components|SkeletalMesh|GetAnimInstance (Variables|Character|GetMesh))))
      (bind _output_get (Variables|Default|SetEnumState (Variables|/Game/Meshes/Final/Enemy_Mesh/ABP_Enemy_Final.ABP_Enemy_Final_C|GetEnum_State _asabp_enemy_final)))
      (switch Utilities|FlowControl|Switch|SwitchonE_Enemy_Animation_State_Final _output_get
        (:NewEnumerator8
          _)
        (:NewEnumerator2
          _))
      (bind _outhit (Collision|LineTraceForObjects _returnvalue (- _returnvalue "0, 0,10.000000") (Utilities|Array|MakeArray "ObjectTypeQuery1" "ObjectTypeQuery2") false 0 "ForDuration"))
      (CallFunction|EnemyFootstepAudio (Variables|/Script/PhysicsCore.PhysicalMaterial|GetSurfaceType (.physmat _outhit))))))

(event OnComponentEndOverlap(GroundDetectionBox)
  (params (OverlappedComponent :type Primitive%20Component%20Object%20Reference) (OtherActor :type Actor%20Object%20Reference) (OtherComp :type Primitive%20Component%20Object%20Reference) (OtherBodyIndex :type Integer))
  ;[0 0 0] Foot Audio TriggerBox
  (Utilities|FlowControl|DoOnce true) ; enters at Reset
)

(event OnComponentEndOverlap(GroundDetectionBox1)
  (params (OverlappedComponent :type Primitive%20Component%20Object%20Reference) (OtherActor :type Actor%20Object%20Reference) (OtherComp :type Primitive%20Component%20Object%20Reference) (OtherBodyIndex :type Integer))
  ;[0 0 0] Foot Audio TriggerBox
  (Utilities|FlowControl|DoOnce true) ; enters at Reset
)

(event Custom|Shoot
  (params (TargetActor :type Actor%20Object%20Reference))
  (Networking|SwitchHasAuthority
    (:Authority
      (Rendering|SetVisibility (Variables|Default|GetPLACEHOLDERSHOOTINGTEXT) true false)
      (CallFunction|EnemyFireAudio)
      (Utilities|FlowControl|Delay 0.5)
      (CallFunction|EnemyFireAudio)
      (Utilities|FlowControl|Delay 0.5)
      (CallFunction|EnemyFireAudio)
      (if (Variables|Default|GetInDarkness)
        (switch int (Math|Random|RandomInteger 6) ; 0-2 = Miss\n3+ = Hit
          (:0
            (Development|PrintString "AI missed their shot" :!label _label))
          (:1
            (goto _label))
          (:2
            (goto _label))
          (:3
            (Class|BPITakeDamage|TakeDamage(Message) TargetActor 20)
            ;[0.1354 0.1354 0.1354] Bean Calling Widget
            (CallFunction|UpdateDamageDirection TargetActor)))
        (Rendering|SetVisibility (Variables|Default|GetPLACEHOLDERSHOOTINGTEXT) false false)
        (else
          (switch int (Math|Random|RandomInteger 4) ; 0-2 = Miss\n3+ = Hit
            (:0
              (Development|PrintString "AI missed their shot" :!label _label_2))
            (:1
              (goto _label_2))
            (:2
              (Class|BPITakeDamage|TakeDamage(Message) TargetActor 20 :!label _label_3)
              (CallFunction|UpdateDamageDirection TargetActor))
            (:3
              (goto _label_3)))
          (Rendering|SetVisibility (Variables|Default|GetPLACEHOLDERSHOOTINGTEXT) false false))))))

(event Custom|PlayerSpotted
  ;[0 0 0] this is for later, probably will need it for sound
)

(event Custom|Stab
  (params (TargetActor :type Actor%20Object%20Reference))
  (Networking|SwitchHasAuthority
    (:Authority
      (Rendering|SetVisibility (Variables|Default|GetPLACEHOLDERSTABBINGTEXT) true false)
      (Utilities|FlowControl|Delay 0.5)
      (Class|BPITakeDamage|TakeDamage(Message) TargetActor 20)
      (CallFunction|UpdateDamageDirection TargetActor)
      (Rendering|SetVisibility (Variables|Default|GetPLACEHOLDERSTABBINGTEXT) false false))))

(event Custom|EnableTurning
  (Variables|Default|SetbUseControllerRotationYaw true))

(event Custom|DisableTurning
  (Variables|Default|SetbUseControllerRotationYaw false))

(event Custom|Enemy_TakeDamage_Audio
  ;[1 0 1] Enemy Audio
  (Audio|PlaySoundatLocation "/Game/SFX/Placeholder_SFX/Grunt_Placeholders/Grunt.Grunt" (Transformation|GetActorLocation) "0, 0, 0" 1.0 1.0 0.0 "/Game/SFX/NewSoundAttenuation.NewSoundAttenuation" 0 0))

(event Custom|Enemy_Footstep_Audio
  (params (SurfaceType :type EPhysicalSurface%20Enum :default "SurfaceType_Default"))
  ;[1 0 1] Enemy Audio
  (bind _returnvalue (Class|FMODBlueprintStatics|PlayEventatLocation (Variables|Audio|GetEnemy_Footstep_Event) (Transformation|GetActorTransform)))
  (bind _returnvalue_2 (Class|FMODBlueprintStatics|EventInstanceIsValid _returnvalue))
  (if _returnvalue_2
    (switch Utilities|FlowControl|Switch|SwitchonEPhysicalSurface SurfaceType
      (:SurfaceType_Default
        (Class|FMODBlueprintStatics|EventInstanceSetParameter _returnvalue "Terrain_Type" 0.0 :!label _label))
      (:SurfaceType4
        (goto _label))
      (:SurfaceType5
        (Class|FMODBlueprintStatics|EventInstanceSetParameter :Name "Terrain_Type" :Value 1.0))
      (:SurfaceType6
        (Class|FMODBlueprintStatics|EventInstanceSetParameter :Name "Terrain_Type" :Value 2.0)))))

(event Custom|Enemy_Fire_Audio
  ;[1 0 1] Enemy Audio
  (bind _returnvalue (Class|FMODBlueprintStatics|PlayEventatLocation (Variables|Audio|GetEnemy_Fire_Event) (Transformation|GetActorTransform)))
  (bind _returnvalue_2 (Class|FMODBlueprintStatics|EventInstanceIsValid _returnvalue))
  (if _returnvalue_2
    (Class|FMODBlueprintStatics|EventInstanceSetParameter _returnvalue "Ammo_Rifle" 1.0)))

(event EventBeginPlay
  (Rendering|SetVisibility (Variables|Default|GetPLACEHOLDERSHOOTINGTEXT) false false)
  (Rendering|SetVisibility (Variables|Default|GetPLACEHOLDERSTABBINGTEXT) false false)
  (bind _returnvalue (Game|SpawnActorfromClass "/Game/Blueprints/Weapons/BPC_Rifle.BPC_Rifle_C" (Math|Transform|MakeTransform "0, 0, 0") "Undefined" 0 true 0 0))
  (Transformation|AttachComponentToComponent _returnvalue (Variables|Character|GetMesh) "Gun_Socket" "SnapToTarget" "SnapToTarget" "SnapToTarget" true))

(event EventTakeDamageActor
  (params (DamageAmount :type Integer) (DamagingPawn :type Pawn%20Object%20Reference))
  (bind _self self)
  ;[0 0 0] Take Damage
  (Networking|SwitchHasAuthority
    (:Authority
      (bind _output_get (Variables|Default|SetHealth (- (Variables|Default|GetHealth) DamageAmount)))
      ;[0 0 0] Check if enemy should be dead
      (if (<= _output_get 0)
        (AI|Components|Blackboard|SetValueasBool (AI|GetBlackboard _self) (Utilities|Name|MakeLiteralName "IsDead") true)
        (Variables|Default|SetInCombat false)
        (bind _asgs_cavalry (Utilities|Casting|CastToGS_Cavalry (Game|GetGameState)))
        (Default|CheckforCombat _asgs_cavalry)
        (else
          (bind _asaic_enemy (Utilities|Casting|CastToAIC_Enemy (AI|GetAIController _self)))
          (Default|UpdateTargetKey _asaic_enemy DamagingPawn)
          (Default|AlertNearby _asaic_enemy DamagingPawn)
          (Variables|Default|SetPlayer DamagingPawn)
          ;[1 0 1] Enemy takes damage Audio
          (CallFunction|EnemyTakeDamageAudio)
          (Utilities|FlowControl|DoOnce false
            (:Completed
              (Variables|Default|SetInCombat true)
              (bind _asgs_cavalry_2 (Utilities|Casting|CastToGS_Cavalry (Game|GetGameState)))
              (Default|CheckforCombat _asgs_cavalry_2))))))))

(fn ConstructionScript)

(fn UpdateDamageDirection
  (params (TargetPlayer :type Actor%20Object%20Reference))
  ;[0.06 0.06 0.06] Logic for Calling Damage Widget
  (bind _asbp_player_character_base (Utilities|Casting|CastToBP_PlayerCharacter_Base TargetPlayer))
  (Utilities|IsValid (Variables|/Game/Blueprints/Characters/BP_PlayerCharacter_Base.BP_PlayerCharacter_Base_C|GetWidgetHandler _asbp_player_character_base)
    (:Is%20Valid
      (Default|DamageSource (Variables|/Game/Blueprints/Characters/BP_PlayerCharacter_Base.BP_PlayerCharacter_Base_C|GetWidgetHandler _asbp_player_character_base) (Transformation|GetWorldLocation (Variables|Collision|GetCapsuleComponent)))
      (return))))