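; GrabbableObject provides grab and release behavior that attaches an object to a given scene component and later detaches it.
; Grab runs only while ComponentActive is true, turning off mesh physics and attaching either the actor's root or the mesh itself, keeping world transform.
; Release sets physics simulation as requested and detaches whichever target the stored UsingRoot flag indicates.
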(event Custom|Grab
  (params (MeshComponent :type Mesh%20Component%20Object%20Reference) (RootActor :type Actor%20Object%20Reference) (AttachTo :type Scene%20Component%20Object%20Reference) (UseRoot :type Boolean))
  (Variables|Default|SetUsingRoot UseRoot)
  (if (Variables|Default|GetComponentActive)
    (bind _output_get (Variables|Default|SetMeshComponent MeshComponent))
    (if (Variables|Default|GetUsingRoot)
      (bind _output_get_2 (Variables|Default|SetRootActor RootActor))
      (Physics|SetSimulatePhysics _output_get false)
      (Transformation|AttachComponentToComponent (VehicleSound|GetRootComponent _output_get_2) AttachTo "None" "KeepWorld" "KeepWorld" "KeepWorld" false)
      (else
        (Physics|SetSimulatePhysics _output_get false)
        (Transformation|AttachComponentToComponent _output_get AttachTo "None" "KeepWorld" "KeepWorld" "KeepWorld" false)))))

(event Custom|Release
  (params (Simulate :type Boolean))
  (Physics|SetSimulatePhysics (Variables|Default|GetMeshComponent) Simulate)
  (if (Variables|Default|GetUsingRoot)
    (Transformation|DetachFromActor (Variables|Default|GetRootActor) "KeepWorld" "KeepWorld" "KeepWorld")
    (else
      (Transformation|DetachFromComponent (Variables|Default|GetMeshComponent) "KeepWorld" "KeepWorld" "KeepWorld" false))))