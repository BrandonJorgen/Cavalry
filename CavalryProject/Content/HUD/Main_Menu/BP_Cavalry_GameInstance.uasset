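; Game instance for Cavalry that manages online sessions, level travel, menu state and player character selection.
; It creates a listen-server session or joins the first one found, and starts levels with a delayed servertravel by index.
; SetGameState swaps deprecated menu and mission-brief actors, or spawns the loading-screen actor.
; It also serves level and character data, matches the current level to its index, and passes the chosen horseman to PlayerState.
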(event Custom|StartNewLevel
  (params (Active%20Level%20Index :type Integer))
  (bind _returnvalue (Game|GetPlayerController 0))
  ;[0 0 0] Starts the Level Corrisponding to the Current Active Level Index
  (Utilities|FlowControl|Delay 0.5)
  ;[0 0 0] Server Travel to next Level via Console Command
  (switch int Active%20Level%20Index
    (:0
      (Development|ExecuteConsoleCommand "servertravel /Game/Levels/MainMenu" _returnvalue))
    (:1
      (Development|ExecuteConsoleCommand "servertravel /Game/Levels/LF-19" _returnvalue))))

(event Custom|StartSession
  ;[0 0 0] Online Session
  (|Session (Game|GetPlayerController 0) 4 false
    (:OnSuccess
      (Development|PrintString "SESSION CREATED")
      (bind _results (|FindSessions 0 1 false)
        (:OnSuccess
          (Variables|Default|SetSession (Utilities|Array|Get(acopy) _results))
          (Game|OpenLevel(byName) "MainMenu" true "?listen"))))
    (:OnFailure
      (Development|PrintString "SESSION CREATION FAILED" true true "(R=1.000000,G=0.000000,B=0.000000,A=1.000000)"))))

(event Custom|JoinSession
  (bind _returnvalue (Game|GetPlayerController 0))
  ;[0 0 0] Online Session
  (bind _results (|FindSessions _returnvalue 1 false)
    (:OnSuccess
      (Development|PrintString (Utilities|String|Append "SESSION FOUND | Server name:  " (Class|FindSessionsCallbackProxy|GetServerName (Utilities|Array|Get(acopy) _results)) " | Current player count: " (Utilities|String|ToString(Integer) (Class|FindSessionsCallbackProxy|GetCurrentPlayers (Utilities|Array|Get(acopy) _results))) " | Max player count: " (Utilities|String|ToString(Integer) (Class|FindSessionsCallbackProxy|GetMaxPlayers (Utilities|Array|Get(acopy) _results))) " | There were " (Utilities|String|ToString(Integer) (Utilities|Array|Length _results)) " other sessions available"))
      (Variables|Default|SetSession (Utilities|Array|Get(acopy) _results))
      (|JoinSession _returnvalue (Utilities|Array|Get(acopy) _results)
        (:OnSuccess
          (Development|PrintString "SESSION JOINED"))
        (:OnFailure
          (Development|PrintString "FAILED TO JOIN FOUND SESSION" true true "(R=1.000000,G=0.000000,B=0.000000,A=1.000000)"))))
    (:OnFailure
      (Development|PrintString "FAILED TO FIND A SESSION" true true "(R=1.000000,G=0.000000,B=0.000000,A=1.000000)"))))

(fn GetLevelData
  ;[0 0 0] Return Level Data for Use in Other Blueprints
  (return (Variables|Config|GetLevel%20Data)))

(fn SetGameState
  (params (NewState :type EGameState%20Enum :default "NewEnumerator1"))
  (bind _missionbrief (Variables|Default|GetMissionBrief))
  (bind _mainmenu (Variables|Default|GetMainMenu))
  ;[0 0 0] Manage Main Menu States (Primarily for having the loading screen show up)
  (if (Utilities|Enum|NotEqual(Enum) NewState (Variables|RuntimeAllocation|GetGame%20State))
    (bind _output_get (Variables|RuntimeAllocation|SetGame%20State NewState))
    (switch Utilities|FlowControl|Switch|SwitchonEGameState _output_get
      (:NewEnumerator1
        (Utilities|IsValid _missionbrief
          (:Is%20Valid
            (Rendering|SetVisibility (Variables|/Game/HUD/Main_Menu/BP_MissionBrief_Actor.BP_MissionBrief_Actor_C|GetStartButton_Widget _missionbrief) true false)
            (CallFunction|MainMenuVisOff))
          (:Is%20Not%20Valid
            (CallFunction|SpawnMissionBrief)
            (CallFunction|MainMenuVisOff))))
      (:NewEnumerator0
        (Utilities|IsValid _mainmenu
          (:Is%20Valid
            (Rendering|SetVisibility (Variables|/Game/HUD/Main_Menu/BP_MainMenu_Actor.BP_MainMenu_Actor_C|GetMM_Center _mainmenu) true false)
            (CallFunction|MissionBriefVisOff))
          (:Is%20Not%20Valid
            (CallFunction|SpawnMainMenu)
            (CallFunction|MissionBriefVisOff))))
      (:NewEnumerator2
        (bind _returnvalue (Game|SpawnActorfromClass "/Game/HUD/Main_Menu/BP_Loading_Actor.BP_Loading_Actor_C" (Math|Transform|MakeTransform "-280.000000, 0,100.000000") "Undefined" 0 0))
        (Variables|Default|SetLoadingScreen _returnvalue)))
    (return true)
    (else
      (return false))))

(fn VerifyActiveLevelIndex
  ;[0 0 0] Checks to Make Sure the Current Level is the ActiveLevelIndex
  (bind _returnvalue (Game|GetCurrentLevelName true))
  (bind _output_get (LocalVariables|SetLocalLevelName (Utilities|String|StringToName _returnvalue)))
  (if (not (Utilities|Name|Equal(Name) _output_get (.FileName (Utilities|Struct|BreakStruc_LevelData (Utilities|Array|Get(acopy) (Variables|Config|GetLevel%20Data))))))
    (bind (_array_element _array_index) (Utilities|Array|ForEachLoopwithBreak (Variables|Config|GetLevel%20Data) :!label _label)
      (:LoopBody
        (if (Utilities|Name|Equal(Name) (LocalVariables|GetLocalLevelName) (.FileName (Utilities|Struct|BreakStruc_LevelData _array_element)))
          (Variables|RuntimeAllocation|SetActive%20Level%20Index _array_index)
          (goto _label Break)))
      (:Completed
        (Development|PrintString (Utilities|String|ToString(Integer) (Variables|RuntimeAllocation|GetActive%20Level%20Index)))))))

(fn SpawnMainMenu
  ;[0.3515 0.2346 0.07227] Spawns the Old Menu (depreciated)
  (bind _returnvalue (Game|SpawnActorfromClass "/Game/HUD/Main_Menu/BP_MainMenu_Actor.BP_MainMenu_Actor_C" (Math|Transform|MakeTransform "-6000.000000, 0,100.000000") "Undefined" 0 0))
  (Variables|Default|SetMainMenu _returnvalue)
  (return))

(fn SpawnMissionBrief
  ;[0.3515 0.2346 0.07227] Spawn the Old Mission Brief Widget (depreciated)
  (bind _returnvalue (Game|SpawnActorfromClass "/Game/HUD/Main_Menu/BP_MissionBrief_Actor.BP_MissionBrief_Actor_C" (Math|Transform|MakeTransform "-6000.000000, 0,100.000000") "Undefined" 0 0))
  (Variables|Default|SetMissionBrief _returnvalue)
  (return))

(fn MainMenuVisOff
  (bind _mainmenu (Variables|Default|GetMainMenu))
  ;[0.3515 0.2346 0.07227] Turns Old Main Menu Widget Off (depreciated)
  (Utilities|IsValid _mainmenu
    (:Is%20Valid
      (Rendering|SetVisibility (Variables|/Game/HUD/Main_Menu/BP_MainMenu_Actor.BP_MainMenu_Actor_C|GetMM_Center _mainmenu) false false))
    (:Is%20Not%20Valid
      _))
  (return))

(fn MissionBriefVisOff
  (bind _missionbrief (Variables|Default|GetMissionBrief))
  ;[0.3515 0.2346 0.07227] Manages Visiablity of the Old 'Get Mission Brief' Button (depreciated)
  (Utilities|IsValid _missionbrief
    (:Is%20Valid
      (Rendering|SetVisibility (Variables|/Game/HUD/Main_Menu/BP_MissionBrief_Actor.BP_MissionBrief_Actor_C|GetStartButton_Widget _missionbrief) false false))
    (:Is%20Not%20Valid
      _))
  (return))

(fn GetCharacterData
  ;[0 0 0] Return Character Data for Use in Other Blueprints
  (return (Variables|Config|GetCharacter_Data)))

(fn SetCharacter
  (params (CharacterIndex :type Integer) (PlayerState :type BP%20Cavalry%20Playerstate%20Object%20Reference))
  (bind _character_data (Variables|Config|GetCharacter_Data))
  (bind _output (Utilities|Array|Get(acopy) _character_data CharacterIndex))
  (bind _character (Utilities|Struct|BreakStruc_CharacterData _output))
  ;[0 0 0] Sets the Character that will Spawn when the next Level Loads
  (Variables|Default|SetPlayerToSpawn _character)
  (if (Utilities|IsValid PlayerState)
    (Variables|/Game/HUD/Main_Menu/Multiplayer_Lobby/BP_CavalryPlayerstate.BP_CavalryPlayerstate_C|SetHorsemenToSpawnAs PlayerState _character))
  (return))