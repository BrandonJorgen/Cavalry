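; Main menu trigger actor that makes the player's widget interaction pointers visible on both motion controllers.
; After a short delay on BeginPlay, it enables query-only collision on its player check component.
; When a BP_PlayerCharacter_Base overlaps that component, it turns on ShowDebug for the left and right controllers' WidgetInteraction components, with no logic to turn it back off.
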(event OnComponentBeginOverlap(Menu_PlayerCheck)
  (params (OverlappedComponent :type Primitive%20Component%20Object%20Reference) (OtherActor :type Actor%20Object%20Reference) (OtherComp :type Primitive%20Component%20Object%20Reference) (OtherBodyIndex :type Integer) (bFromSweep :type Boolean) (SweepResult :type Hit%20Result%20Structure%20%28by%20ref%29))
  (bind _asbp_player_character_base (Utilities|Casting|CastToBP_PlayerCharacter_Base OtherActor))
  (Variables|/Script/UMG.WidgetInteractionComponent|SetbShowDebug (Variables|/Game/VirtualRealityBP/Blueprints/BP_MotionController.BP_MotionController_C|GetWidgetInteraction (Variables|/Game/Blueprints/Characters/BP_PlayerCharacter_Base.BP_PlayerCharacter_Base_C|GetRight%20Controller _asbp_player_character_base)) true)
  (Variables|/Script/UMG.WidgetInteractionComponent|SetbShowDebug (Variables|/Game/VirtualRealityBP/Blueprints/BP_MotionController.BP_MotionController_C|GetWidgetInteraction (Variables|/Game/Blueprints/Characters/BP_PlayerCharacter_Base.BP_PlayerCharacter_Base_C|GetLeft%20Controller _asbp_player_character_base)) true))

(event EventBeginPlay
  (Utilities|FlowControl|Delay 2.0)
  (Collision|SetCollisionEnabled (Variables|Default|GetMenu_PlayerCheck) "QueryOnly"))

(fn ConstructionScript)