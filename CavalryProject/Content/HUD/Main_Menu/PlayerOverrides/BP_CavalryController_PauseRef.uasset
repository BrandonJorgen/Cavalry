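; VR player controller that routes motion-controller input to the possessed horseman or base player character, cached on BeginPlay.
; Thumbsticks drive movement, strafing, deadzone-gated single-step turning, night vision and objective display.
; Each hand grabs, fires, changes firemode or activates tools, and releases magazines on its held actor.
; The menu button toggles the pause menu and widget-pointer debug display, while triggers also click UI through each hand's widget interaction.
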(event EventBeginPlay
  (bind _returnvalue (Pawn|GetControlledPawn))
  (Utilities|FlowControl|Sequence
    (:then_0
      ;[0 0 0] Grabbing the character that this controller possesses
      (Utilities|FlowControl|Sequence
        (:then_0
          (bind _asbpc_conquest (Utilities|Casting|CastToBPC_Conquest _returnvalue))
          (Utilities|IsValid _asbpc_conquest
            (:Is%20Valid
              (Variables|Default|SetpossessedCharacter _asbpc_conquest))))
        (:then_1
          (bind _asbpc_war (Utilities|Casting|CastToBPC_War _returnvalue))
          (Utilities|IsValid _asbpc_war
            (:Is%20Valid
              (Variables|Default|SetpossessedCharacter _asbpc_war))))
        (:then_2
          (bind _asbpc_death (Utilities|Casting|CastToBPC_Death _returnvalue))
          (Utilities|IsValid _asbpc_death
            (:Is%20Valid
              (Variables|Default|SetpossessedCharacter _asbpc_death))))
        (:then_3
          (bind _asbpc_famine (Utilities|Casting|CastToBPC_Famine _returnvalue))
          (Utilities|IsValid _asbpc_famine
            (:Is%20Valid
              (Variables|Default|SetpossessedCharacter _asbpc_famine))))
        (:then_4
          (bind _asbp_player_character_base (Utilities|Casting|CastToBP_PlayerCharacter_Base _returnvalue))
          (Utilities|IsValid _asbp_player_character_base
            (:Is%20Valid
              (Variables|Default|SetpossessedCharacter _asbp_player_character_base))))))
    (:then_1
      (if (Variables|Default|GetTreadmillEnabled)
        _))))

(event Input|ActionEvents|InputActionGrabLeft
  (params (Key :type Key%20Structure :default "None"))
  (bind _possessedcharacter (Variables|Default|GetpossessedCharacter))
  (bind _left_controller (Variables|/Game/Blueprints/Characters/BP_PlayerCharacter_Base.BP_PlayerCharacter_Base_C|GetLeft%20Controller _possessedcharacter))
  ;[0 0 0] Player Input
  ;;[0.1095 0.1095 0.1095] Left Grabbing
  (:Pressed
    (Default|GrabActor _left_controller))
  (:Released
    (Default|ReleaseActor _left_controller)))

(event Input|ActionEvents|InputActionSecondaryMenuButton
  (params (Key :type Key%20Structure :default "None"))
  (bind _possessedcharacter (Variables|Default|GetpossessedCharacter))
  (bind _left_controller (Variables|/Game/Blueprints/Characters/BP_PlayerCharacter_Base.BP_PlayerCharacter_Base_C|GetLeft%20Controller _possessedcharacter))
  (bind _right_controller (Variables|/Game/Blueprints/Characters/BP_PlayerCharacter_Base.BP_PlayerCharacter_Base_C|GetRight%20Controller _possessedcharacter))
  (bind _widgethandler (Variables|/Game/Blueprints/Characters/BP_PlayerCharacter_Base.BP_PlayerCharacter_Base_C|GetWidgetHandler _possessedcharacter))
  (bind _widgetinteraction (Variables|/Game/VirtualRealityBP/Blueprints/BP_MotionController.BP_MotionController_C|GetWidgetInteraction _right_controller))
  (bind _widgetinteraction_2 (Variables|/Game/VirtualRealityBP/Blueprints/BP_MotionController.BP_MotionController_C|GetWidgetInteraction _left_controller))
  ;[0 0 0] Player Input
  ;;[0.1095 0.1095 0.1095] Pause Menu
  (:Pressed
    (if (Variables|Default|GetMenuOn?)
      (Default|PauseMenuOff _widgethandler)
      (Variables|/Script/UMG.WidgetInteractionComponent|SetbShowDebug _widgetinteraction false)
      (Variables|/Script/UMG.WidgetInteractionComponent|SetbShowDebug _widgetinteraction_2 false)
      (Variables|Default|SetMenuOn? false)
      (else
        (Default|PauseMenuon _widgethandler)
        (Variables|/Script/UMG.WidgetInteractionComponent|SetbShowDebug _widgetinteraction true)
        (Variables|/Script/UMG.WidgetInteractionComponent|SetbShowDebug _widgetinteraction_2 true)
        (Variables|Default|SetMenuOn? true)))))

(event Input|ActionEvents|InputActionPrimaryTriggerLeft
  (params (Key :type Key%20Structure :default "None"))
  (bind _possessedcharacter (Variables|Default|GetpossessedCharacter))
  (bind _left_controller (Variables|/Game/Blueprints/Characters/BP_PlayerCharacter_Base.BP_PlayerCharacter_Base_C|GetLeft%20Controller _possessedcharacter))
  (bind _widgetinteraction (Variables|/Game/VirtualRealityBP/Blueprints/BP_MotionController.BP_MotionController_C|GetWidgetInteraction _left_controller))
  ;[0 0 0] Player Input
  ;;[0.1095 0.1095 0.1095] Fire Weapon Left
  (:Pressed
    (CallFunction|ManageLeftHWidInteract true _widgetinteraction)
    (bind _asbp_firearm_base (Utilities|Casting|CastToBP_Firearm_Base (Variables|/Game/VirtualRealityBP/Blueprints/BP_MotionController.BP_MotionController_C|GetAttachedActor _left_controller)))
    (Utilities|FlowControl|DoOnce false :!label _label
      (:Completed
        (Class|BPIWeaponControls|Shoot(Message) _asbp_firearm_base "NewEnumerator1"))))
  (:Released
    (CallFunction|ManageLeftHWidInteract false _widgetinteraction)
    (Class|BPIWeaponControls|ShootRelease(Message) _asbp_firearm_base)
    (goto _label Reset)))

(event Input|ActionEvents|InputActionPrimaryTriggerRight
  (params (Key :type Key%20Structure :default "None"))
  (bind _possessedcharacter (Variables|Default|GetpossessedCharacter))
  (bind _right_controller (Variables|/Game/Blueprints/Characters/BP_PlayerCharacter_Base.BP_PlayerCharacter_Base_C|GetRight%20Controller _possessedcharacter))
  (bind _widgetinteraction (Variables|/Game/VirtualRealityBP/Blueprints/BP_MotionController.BP_MotionController_C|GetWidgetInteraction _right_controller))
  ;[0 0 0] Player Input
  ;;[0.1095 0.1095 0.1095] Fire Weapon Right
  (:Pressed
    (CallFunction|ManageRightHWidInteract true _widgetinteraction)
    (bind _asbp_firearm_base (Utilities|Casting|CastToBP_Firearm_Base (Variables|/Game/VirtualRealityBP/Blueprints/BP_MotionController.BP_MotionController_C|GetAttachedActor _right_controller)))
    (Utilities|FlowControl|DoOnce false :!label _label
      (:Completed
        (Class|BPIWeaponControls|Shoot(Message) _asbp_firearm_base "NewEnumerator0"))))
  (:Released
    (CallFunction|ManageRightHWidInteract false _widgetinteraction)
    (Class|BPIWeaponControls|ShootRelease(Message) _asbp_firearm_base)
    (goto _label Reset)))

(event Input|ActionEvents|InputActionGrabRight
  (params (Key :type Key%20Structure :default "None"))
  (bind _possessedcharacter (Variables|Default|GetpossessedCharacter))
  (bind _right_controller (Variables|/Game/Blueprints/Characters/BP_PlayerCharacter_Base.BP_PlayerCharacter_Base_C|GetRight%20Controller _possessedcharacter))
  ;[0 0 0] Player Input
  ;;[0.1095 0.1095 0.1095] Right Grabbing
  (:Pressed
    (Default|GrabActor _right_controller))
  (:Released
    (Default|ReleaseActor _right_controller)))

(event Input|ActionEvents|InputActionSecondaryButtonLeft
  (params (Key :type Key%20Structure :default "None"))
  (bind _possessedcharacter (Variables|Default|GetpossessedCharacter))
  (bind _left_controller (Variables|/Game/Blueprints/Characters/BP_PlayerCharacter_Base.BP_PlayerCharacter_Base_C|GetLeft%20Controller _possessedcharacter))
  (bind _attachedactor (Variables|/Game/VirtualRealityBP/Blueprints/BP_MotionController.BP_MotionController_C|GetAttachedActor _left_controller))
  (:Pressed
    (if (Utilities|IsValid _attachedactor)
      (bind _asbp_firearm_base (Utilities|Casting|CastToBP_Firearm_Base _attachedactor)
        (:then
          (Class|BPIWeaponControls|ChangeFiremode(Message) _asbp_firearm_base))
        (:CastFailed
          (bind _asbp_tool_base (Utilities|Casting|CastToBP_Tool_Base _attachedactor))
          (Default|ActivateTool _asbp_tool_base true))))))

(event Input|ActionEvents|InputActionPrimaryButtonRight
  (params (Key :type Key%20Structure :default "None"))
  (bind _possessedcharacter (Variables|Default|GetpossessedCharacter))
  (bind _right_controller (Variables|/Game/Blueprints/Characters/BP_PlayerCharacter_Base.BP_PlayerCharacter_Base_C|GetRight%20Controller _possessedcharacter))
  (bind _attachedactor (Variables|/Game/VirtualRealityBP/Blueprints/BP_MotionController.BP_MotionController_C|GetAttachedActor _right_controller))
  (:Pressed
    (if (Utilities|IsValid _attachedactor)
      (bind _asbp_firearm_base (Utilities|Casting|CastToBP_Firearm_Base _attachedactor))
      (Class|BPIWeaponControls|ReleaseMagazine(Message) _asbp_firearm_base))))

(event Input|ActionEvents|InputActionSecondaryButtonRight
  (params (Key :type Key%20Structure :default "None"))
  (bind _possessedcharacter (Variables|Default|GetpossessedCharacter))
  (bind _right_controller (Variables|/Game/Blueprints/Characters/BP_PlayerCharacter_Base.BP_PlayerCharacter_Base_C|GetRight%20Controller _possessedcharacter))
  (bind _attachedactor (Variables|/Game/VirtualRealityBP/Blueprints/BP_MotionController.BP_MotionController_C|GetAttachedActor _right_controller))
  (:Pressed
    (if (Utilities|IsValid _attachedactor)
      (bind _asbp_firearm_base (Utilities|Casting|CastToBP_Firearm_Base _attachedactor)
        (:then
          (Class|BPIWeaponControls|ChangeFiremode(Message) _asbp_firearm_base))
        (:CastFailed
          (bind _asbp_tool_base (Utilities|Casting|CastToBP_Tool_Base _attachedactor))
          (Default|ActivateTool _asbp_tool_base true))))))

(event Input|ActionEvents|InputActionThumbstickPressLeft
  (params (Key :type Key%20Structure :default "None"))
  ;[0 0 0] Player Input
  ;;[0.1095 0.1095 0.1095] Nightvision
  (:Pressed
    (Default|NightVisionTrigger (Variables|Default|GetpossessedCharacter))))

(event Input|ActionEvents|InputActionThumbstickPressRight
  (params (Key :type Key%20Structure :default "None"))
  (bind _possessedcharacter (Variables|Default|GetpossessedCharacter))
  (bind _widgethandler (Variables|/Game/Blueprints/Characters/BP_PlayerCharacter_Base.BP_PlayerCharacter_Base_C|GetWidgetHandler _possessedcharacter))
  (bind _cur_objectivedis (Variables|/Game/HUD/Widgets/Damage_Display/BP_HorsemenHUD.BP_HorsemenHUD_C|GetCur_ObjectiveDis _widgethandler))
  ;[0 0 0] Player Input
  ;;[0.1095 0.1095 0.1095] Display Objective
  (:Pressed
    (Default|TempDisplayObejctive _widgethandler)
    (if (Utilities|IsValid _cur_objectivedis)
      (Default|TempDisplayObejctive _cur_objectivedis))))

(event Input|ActionEvents|InputActionPrimaryButtonLeft
  (params (Key :type Key%20Structure :default "None"))
  (bind _possessedcharacter (Variables|Default|GetpossessedCharacter))
  (bind _left_controller (Variables|/Game/Blueprints/Characters/BP_PlayerCharacter_Base.BP_PlayerCharacter_Base_C|GetLeft%20Controller _possessedcharacter))
  (bind _attachedactor (Variables|/Game/VirtualRealityBP/Blueprints/BP_MotionController.BP_MotionController_C|GetAttachedActor _left_controller))
  (:Pressed
    (if (Utilities|IsValid _attachedactor)
      (bind _asbp_firearm_base (Utilities|Casting|CastToBP_Firearm_Base _attachedactor))
      (Class|BPIWeaponControls|ReleaseMagazine(Message) _asbp_firearm_base))))

(event Input|AxisEvents|InputAxisMotionControllerThumbLeft_X
  (params (AxisValue :type Float%20%28single-precision%29))
  ;[0 0 0] Player Input
  ;;[0.1095 0.1095 0.1095] Left/Right Movement
  (Default|Strafe (Variables|Default|GetpossessedCharacter) AxisValue))

(event Input|AxisEvents|InputAxisMotionControllerThumbLeft_Y
  (params (AxisValue :type Float%20%28single-precision%29))
  ;[0 0 0] Player Input
  ;;[0.1095 0.1095 0.1095] Forward/Backward Movement
  (Default|Movement (Variables|Default|GetpossessedCharacter) AxisValue))

(event Input|AxisEvents|InputAxisMotionControllerThumbRight_X
  (params (AxisValue :type Float%20%28single-precision%29))
  ;[0 0 0] Player Input
  ;;[0.1095 0.1095 0.1095] Rotation
  (if (>= (Math|Float|Absolute(Float) AxisValue) (Variables|Default|GetTurn%20Deadzone))
    (Utilities|FlowControl|DoOnce false :!label _label
      (:Completed
        (Default|Rotation (Variables|Default|GetpossessedCharacter) AxisValue)))
    (else
      (goto _label Reset))))

(fn ConstructionScript)

(fn ManageRightHWidInteract
  (params (Pressed? :type Boolean) (Wid_Interaction :type Widget%20Interaction%20Component%20Object%20Reference))
  (if Pressed?
    (Class|WidgetInteractionComponent|PressPointerKey Wid_Interaction "LeftMouseButton")
    (else
      (Class|WidgetInteractionComponent|ReleasePointerKey Wid_Interaction "LeftMouseButton"))))

(fn ManageLeftHWidInteract
  (params (Pressed? :type Boolean) (Wid_Interaction :type Widget%20Interaction%20Component%20Object%20Reference))
  (if Pressed?
    (if (== (Variables|/Script/UMG.WidgetInteractionComponent|GetPointerIndex Wid_Interaction) 0)
      (Variables|/Script/UMG.WidgetInteractionComponent|SetPointerIndex Wid_Interaction 1))
    (Class|WidgetInteractionComponent|PressPointerKey Wid_Interaction "LeftMouseButton")
    (else
      (Class|WidgetInteractionComponent|ReleasePointerKey Wid_Interaction "LeftMouseButton"))))