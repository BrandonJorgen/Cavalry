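; BP_LevelSelector is a physical VR menu where motion controllers touch collision volumes to pick and start a level.
; Back and Forward volumes cycle SelectedLevel with wraparound through the game instance's LevelData, updating the Widget_SelectedLevel image and name.
; The Start volume swaps in a Yes/No confirmation popup by toggling visibility and collision.
; Yes sets the game state and calls StartNewLevel on the game instance, while No restores the Start button.
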(event OnComponentBeginOverlap(BackCollision)
  (params (OverlappedComponent :type Primitive%20Component%20Object%20Reference) (OtherActor :type Actor%20Object%20Reference) (OtherComp :type Primitive%20Component%20Object%20Reference) (OtherBodyIndex :type Integer) (bFromSweep :type Boolean) (SweepResult :type Hit%20Result%20Structure%20%28by%20ref%29))
  (bind _gameinstance (Variables|Default|GetGameInstance))
  (bind _level_data (Variables|/Game/HUD/Main_Menu/BP_Cavalry_GameInstance.BP_Cavalry_GameInstance_C|GetLevel%20Data _gameinstance))
  (Utilities|Casting|CastToBP_MotionController OtherActor)
  (if (< (- (Variables|Default|GetSelectedLevel) 1) 0)
    (Variables|Default|SetSelectedLevel (- (Utilities|Array|Length _level_data) 1))
    (else
      (bind _output_get (Variables|Default|SetSelectedLevel (- (Variables|Default|GetSelectedLevel) 1)))))
  (Default|UpdateImage (Variables|Default|GetWidgSelLevel) (.Image (Utilities|Struct|BreakStruc_LevelData (Utilities|Array|Get(acopy) _level_data _output_get))) (.DisplayName (Utilities|Struct|BreakStruc_LevelData (Utilities|Array|Get(acopy) _level_data _output_get)))))

(event OnComponentBeginOverlap(ForwardCollision)
  (params (OverlappedComponent :type Primitive%20Component%20Object%20Reference) (OtherActor :type Actor%20Object%20Reference) (OtherComp :type Primitive%20Component%20Object%20Reference) (OtherBodyIndex :type Integer) (bFromSweep :type Boolean) (SweepResult :type Hit%20Result%20Structure%20%28by%20ref%29))
  (bind _gameinstance (Variables|Default|GetGameInstance))
  (bind _level_data (Variables|/Game/HUD/Main_Menu/BP_Cavalry_GameInstance.BP_Cavalry_GameInstance_C|GetLevel%20Data _gameinstance))
  (Utilities|Casting|CastToBP_MotionController OtherActor)
  (if (> (+ (Variables|Default|GetSelectedLevel) 1) (- (Utilities|Array|Length _level_data) 1))
    (bind _output_get (Variables|Default|SetSelectedLevel 0))
    (else
      (Variables|Default|SetSelectedLevel (+ (Variables|Default|GetSelectedLevel) 1))))
  (Default|UpdateImage (Variables|Default|GetWidgSelLevel) (.Image (Utilities|Struct|BreakStruc_LevelData (Utilities|Array|Get(acopy) _level_data _output_get))) (.DisplayName (Utilities|Struct|BreakStruc_LevelData (Utilities|Array|Get(acopy) _level_data _output_get)))))

(event OnComponentBeginOverlap(StartLevelCollision)
  (params (OverlappedComponent :type Primitive%20Component%20Object%20Reference) (OtherActor :type Actor%20Object%20Reference) (OtherComp :type Primitive%20Component%20Object%20Reference) (OtherBodyIndex :type Integer) (bFromSweep :type Boolean) (SweepResult :type Hit%20Result%20Structure%20%28by%20ref%29))
  (bind _start_level_collision (Variables|Default|GetStart%20Level%20Collision))
  (Utilities|Casting|CastToBP_MotionController OtherActor)
  (Rendering|SetVisibility (Variables|Default|GetConfirmation%20Popup) true true)
  (Collision|SetCollisionEnabled (Variables|Default|GetYes%20Collision) "QueryAndPhysics")
  (Rendering|SetVisibility _start_level_collision false true)
  (Collision|SetCollisionEnabled _start_level_collision "NoCollision"))

(event OnComponentBeginOverlap(YesCollision)
  (params (OverlappedComponent :type Primitive%20Component%20Object%20Reference) (OtherActor :type Actor%20Object%20Reference) (OtherComp :type Primitive%20Component%20Object%20Reference) (OtherBodyIndex :type Integer) (bFromSweep :type Boolean) (SweepResult :type Hit%20Result%20Structure%20%28by%20ref%29))
  (bind _gameinstance (Variables|Default|GetGameInstance))
  (Utilities|Casting|CastToBP_MotionController OtherActor)
  (Default|SetGameState _gameinstance "NewEnumerator2")
  (Default|StartNewLevel _gameinstance (Variables|Default|GetSelectedLevel)))

(event OnComponentBeginOverlap(NoCollision)
  (params (OverlappedComponent :type Primitive%20Component%20Object%20Reference) (OtherActor :type Actor%20Object%20Reference) (OtherComp :type Primitive%20Component%20Object%20Reference) (OtherBodyIndex :type Integer) (bFromSweep :type Boolean) (SweepResult :type Hit%20Result%20Structure%20%28by%20ref%29))
  (bind _start_level_collision (Variables|Default|GetStart%20Level%20Collision))
  (Utilities|Casting|CastToBP_MotionController OtherActor)
  (Rendering|SetVisibility (Variables|Default|GetConfirmation%20Popup) false true)
  (Collision|SetCollisionEnabled (Variables|Default|GetYes%20Collision) "NoCollision")
  (Rendering|SetVisibility _start_level_collision true true)
  (Collision|SetCollisionEnabled _start_level_collision "QueryAndPhysics"))

(event EventBeginPlay
  (Rendering|SetVisibility (Variables|Default|GetConfirmation%20Popup) false true)
  (Collision|SetCollisionEnabled (Variables|Default|GetYes%20Collision) "NoCollision")
  (bind _asbp_cavalry_game_instance (Utilities|Casting|CastToBP_Cavalry_GameInstance (Game|GetGameInstance)))
  (Variables|Default|SetGameInstance _asbp_cavalry_game_instance)
  (bind _aswidget_selected_level (Utilities|Casting|CastToWidget_SelectedLevel (UserInterface|GetWidget (Variables|Default|GetCurrentLevelSelected))))
  (bind _output_get (Variables|Default|SetWidgSelLevel _aswidget_selected_level))
  (Default|UpdateImage _output_get (.Image (Utilities|Struct|BreakStruc_LevelData (Utilities|Array|Get(acopy) (Variables|/Game/HUD/Main_Menu/BP_Cavalry_GameInstance.BP_Cavalry_GameInstance_C|GetLevel%20Data _asbp_cavalry_game_instance) (Variables|Default|GetSelectedLevel)))) (.DisplayName (Utilities|Struct|BreakStruc_LevelData (Utilities|Array|Get(acopy) (Variables|/Game/HUD/Main_Menu/BP_Cavalry_GameInstance.BP_Cavalry_GameInstance_C|GetLevel%20Data _asbp_cavalry_game_instance) (Variables|Default|GetSelectedLevel))))))

(fn ConstructionScript)