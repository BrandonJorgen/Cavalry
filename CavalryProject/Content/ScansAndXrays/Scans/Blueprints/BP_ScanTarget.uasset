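; BP_ScanTarget is a scan target actor that displays the player's distance to it in meters on a widget.
; Every Tick it casts its Widget component's user widget to 3DWIDGET, measures the distance from player character 0 to the actor, and converts it to meters.
; It writes that value, suffixed with "M", into the widget's MetersCounter text.
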(event EventTick
  (params (DeltaSeconds :type Float%20%28single-precision%29))
  ;[1 0.6939 0] MetersCounter
  (bind _as3dwidget (Utilities|Casting|CastTo3DWIDGET (UserInterface|GetUserWidgetObject (Variables|Default|GetWidget))))
  (Rendering|Components|TextRender|SetText (Variables|/Game/ScansAndXrays/Scans/Blueprints/3DWIDGET.3DWIDGET_C|GetMetersCounter _as3dwidget) (Utilities|Text|ToText(String) (Utilities|String|Append (Utilities|String|ToString(Integer) (/ (Math|Float|Round (Math|Vector|Distance(Vector) (Transformation|GetActorLocation (Game|GetPlayerCharacter 0)) (Transformation|GetActorLocation))) 100)) " M"))))

(fn ConstructionScript)